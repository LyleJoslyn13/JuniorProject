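; BP_TrashCan1 is an item pickup that hands the player a random power-up.
; On BeginPlay it rolls an E_PowerUps value, with the range starting past index 0, and sets the matching item mesh.
; Tick spins the mesh around yaw by a fixed step per frame.
; When a BP_Character_Player overlaps the collision box, it passes the selection to OnItemPickup and destroys itself.
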(event OnComponentBeginOverlap(CollisionBox)
  (params (OverlappedComponent :type Primitive%20Component%20Object%20Reference) (OtherActor :type Actor%20Object%20Reference) (OtherComp :type Primitive%20Component%20Object%20Reference) (OtherBodyIndex :type Integer) (bFromSweep :type Boolean) (SweepResult :type Hit%20Result%20Structure%20%28by%20ref%29))
  ;[1 0 0.005823] Tells player what item was stored
  (if (Class|GameplayStatics|ObjectIsA OtherActor "/Game/Characters/Player/Character/BP_Character_Player.BP_Character_Player_C")
    (bind _asbp_character_player (Utilities|Casting|CastToBP_Character_Player OtherActor))
    (Default|OnItemPickup _asbp_character_player (Variables|Default|GetItemSelection))
    (Actor|DestroyActor)))

(event Collision|EventActorBeginOverlap
  (params (OtherActor :type Actor%20Object%20Reference)))

(event EventTick
  (params (DeltaSeconds :type Float%20%28single-precision%29))
  (bind _itemmesh (Variables|Default|GetItemMesh))
  (bind _relativerotation (Variables|/Script/Engine.SceneComponent|GetRelativeRotation _itemmesh))
  (Transformation|SetRelativeRotation _itemmesh (Math|Rotator|MakeRotator (.roll _relativerotation) (.pitch _relativerotation) (+ (.yaw _relativerotation) 1.0)) false false))

(event EventBeginPlay
  (bind _output_get (Variables|Default|SetItemSelection (Utilities|Enum|ByteToEnumE_PowerUps (Math|Conversions|ToByte(Integer) (Math|Random|RandomIntegerinRange 1 (- (|GetNumEnumEntries) 1))))))
  (Components|StaticMesh|SetStaticMesh (Variables|Default|GetItemMesh) (Utilities|Select :Index _output_get :NewEnumerator8 "/Game/StarterContent/Shapes/Shape_Cube.Shape_Cube" :NewEnumerator0 "/Game/ItemSystem/Mesh/SM_Plow.SM_Plow" :NewEnumerator3 "/Game/ItemSystem/Mesh/SM_Turret.SM_Turret" :NewEnumerator1 "/Game/ItemSystem/Mesh/SM_ExplosivePumpkin.SM_ExplosivePumpkin" :NewEnumerator2 "/Game/ItemSystem/Mesh/SM_BrokenInstrument.SM_BrokenInstrument" :NewEnumerator4 "/Game/ItemSystem/Mesh/SM_BombBoost.SM_BombBoost" :NewEnumerator5 "/Game/ItemSystem/Mesh/SM_ShrinkingPotion.SM_ShrinkingPotion" :NewEnumerator6 "/Game/ItemSystem/Mesh/SM_EnlargementPotion.SM_EnlargementPotion" :NewEnumerator7 "/Game/ItemSystem/Mesh/SM_InvisibilityPotion.SM_InvisibilityPotion" :NewEnumerator9 "/Game/ItemSystem/Mesh/SM_Repair.SM_Repair" :NewEnumerator10 "/Game/ItemSystem/Mesh/SM_Umbrella.SM_Umbrella" :NewEnumerator11 "/Game/ItemSystem/Mesh/SM_SlingShot.SM_SlingShot" :NewEnumerator12 "/Game/ItemSystem/Mesh/SM_BaseBallBat.SM_BaseBallBat" :NewEnumerator13 "/Game/ItemSystem/Mesh/SM_TennisRacket.SM_TennisRacket")))

(fn ConstructionScript)