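; BP_Weapon_BaseballBat is a melee bat weapon that tracks when its owning character is swinging it.
; Firing sets IsSwinging and the weapon state, and the character's animation-complete event clears the swing flag.
; The component hit event is empty.
; Disconnected logic would print the name of a struck non-owner actor and apply a scaled velocity-change impulse to its head bone, but never runs.
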(event OnComponentHit(Weapon)
  (params (HitComponent :type Primitive%20Component%20Object%20Reference) (OtherActor :type Actor%20Object%20Reference) (OtherComp :type Primitive%20Component%20Object%20Reference) (NormalImpulse :type Vector :default "0, 0, 0") (Hit :type Hit%20Result%20Structure%20%28by%20ref%29)))

(event EventCharacterAnimationComplete
  (Variables|Default|SetisSwinging false))

(event EventPlayerFireWeapon
  (params (attackTarget :type Actor%20Object%20Reference) (attackPower :type Float%20%28double-precision%29))
  (Variables|Default|SetisSwinging true)
  (Variables|Default|SetweaponStates "NewEnumerator0"))

(fn ConstructionScript
  (|CallParentFunction))