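; Pumpkin bomb weapon that the owning character throws as an arcing projectile, with speed scaled by attack power.
; On fire it breaks the right-hand physics constraint and traces from the camera to aim from the projectile arrow.
; It spawns the projectile through the attack component's Trashball function, then attaches the weapon to that projectile's collision box.
; Impulse, constraint and collision-response nodes are left unconnected.
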(event EventPlayerFireWeapon
  (params (attackTarget :type Actor%20Object%20Reference) (attackPower :type Float%20%28double-precision%29))
  (bind _projectilearrow (Variables|Default|GetProjectileArrow))
  (bind _camerareference (Variables|Default|GetcameraReference))
  (bind _returnvalue (Transformation|GetWorldLocation _projectilearrow))
  (bind _returnvalue_2 (Transformation|GetWorldLocation _camerareference))
  (Class|PhysicsConstraintComponent|BreakConstraint (Variables|/Game/Characters/CharacterBase/BP_Character_Base.BP_Character_Base_C|GetPC_Hand_r (Variables|Default|GetowningCharacter)))
  (bind _outhit (Collision|LineTraceByChannel _returnvalue_2 (+ _returnvalue_2 (* (Math|Vector|GetForwardVector _camerareference) 5e+03)) "TraceTypeQuery1" false 0 "None"))
  (Default|Trashball (Variables|Default|GetBPC_Attacks) (Math|Transform|MakeTransform _returnvalue (Math|Conversions|RotationFromXVector (Math|Vector|GetUnitDirection(Vector) _returnvalue (Math|Vector|SelectVector (.Location (Collision|BreakHitResult _outhit)) (.TraceEnd (Collision|BreakHitResult _outhit)) (.bBlockingHit (Collision|BreakHitResult _outhit))))) "1.000000,1.000000,1.000000") self 0 (Utilities|Struct|MakeS_DamageInfo 25.0 "NewEnumerator2") (Math|Float|MapRangeClamped attackPower 0.0 1.0 1e+03 4e+03) 1.0)
  (Transformation|AttachComponentToComponent (Variables|Default|GetWeapon) (Variables|/Game/Universal_Systems/Projectiles/BP_Projectile_Base.BP_Projectile_Base_C|GetBoxCollision (Variables|/Game/Universal_Systems/DamageSystem/BPC_Attacks.BPC_Attacks_C|Gettrashballref (Variables|Default|GetBPC_Attacks))) "None" "KeepWorld" "KeepWorld" "KeepWorld" true))

(fn ConstructionScript
  (|CallParentFunction))