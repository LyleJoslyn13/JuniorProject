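; Throwable explosive pumpkin weapon whose light pulses with its audio's envelope data and resets when playback ends.
; Firing aims by camera trace, spawns a power-scaled Trashball projectile, drops the pumpkin and physics-constrains it to that projectile, adjusting collision for cart-riding throwers.
; Hitting anything but the thrower destroys the projectile and triggers Explode, which spawns a fracture actor and master field before running the parent explosion.
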(event OnComponentHit(Weapon)
  (params (HitComponent :type Primitive%20Component%20Object%20Reference) (OtherActor :type Actor%20Object%20Reference) (OtherComp :type Primitive%20Component%20Object%20Reference) (NormalImpulse :type Vector :default "0, 0, 0") (Hit :type Hit%20Result%20Structure%20%28by%20ref%29))
  (if (Variables|Default|GetisThrown)
    (if (!= (Variables|Default|GetownerToIgnoreAfterDrop) OtherActor)
      (Utilities|FlowControl|DoOnce false
        (:Completed
          (Class|PhysicsConstraintComponent|BreakConstraint (Variables|Default|GetPC_PumpkinToProjectile))
          (Actor|DestroyActor (Variables|/Game/Universal_Systems/DamageSystem/BPC_Attacks.BPC_Attacks_C|GetprojectileRef (Variables|Default|GetBPC_Attacks)))
          (CallFunction|Explode))))))

(event Custom|OnAudioPlayback
  (params (PlayingSoundWave :type Sound%20Wave%20Object%20Reference) (PlaybackPercent :type Float%20%28single-precision%29))
  (bind _outenvelopedata (Class|AudioComponent|GetCookedEnvelopeData (Variables|Default|GetWeapon_Audio)))
  (Rendering|Components|Light|SetLightColor (Variables|Default|GetPumpkinLight) (* (* _outenvelopedata 5e+02) (Variables|Default|GetoriginalLightColor)) true)
  (Rendering|Components|Light|SetIntensity (Variables|Default|GetPumpkinLight) (* (* _outenvelopedata 1e+01) (Variables|Default|GetoriginalLightIntensity))))

(event Custom|OnAudioFinished
  (Rendering|Components|Light|SetLightColor (Variables|Default|GetPumpkinLight) (Variables|Default|GetoriginalLightColor) true)
  (Rendering|Components|Light|SetIntensity (Variables|Default|GetPumpkinLight) (Variables|Default|GetoriginalLightIntensity)))

(event EventBeginPlay
  (bind _pumpkinlight (Variables|Default|GetPumpkinLight))
  (|CallParentFunction)
  (Variables|Default|SetoriginalLightColor (Rendering|Components|Light|GetLightColor _pumpkinlight))
  (Variables|Default|SetoriginalLightIntensity (Variables|/Script/Engine.LightComponentBase|GetIntensity _pumpkinlight))
  (EventDispatchers|BindEventtoOnAudioPlaybackPercent (Variables|Default|GetWeapon_Audio) (delegate Custom|OnAudioPlayback))
  (EventDispatchers|AssignOnAudioFinished (Variables|Default|GetWeapon_Audio) (delegate Custom|OnAudioFinished)))

(event EventPlayerFireWeapon
  (params (attackTarget :type Actor%20Object%20Reference) (attackPower :type Float%20%28double-precision%29))
  (bind _bpc_attacks (Variables|Default|GetBPC_Attacks))
  (bind _projectilearrow (Variables|Default|GetProjectileArrow))
  (bind _camerareference (Variables|Default|GetcameraReference))
  (bind _returnvalue (Transformation|GetWorldLocation _projectilearrow))
  (bind _returnvalue_2 (Transformation|GetWorldLocation _camerareference))
  (bind _projectileref (Variables|/Game/Universal_Systems/DamageSystem/BPC_Attacks.BPC_Attacks_C|GetprojectileRef _bpc_attacks))
  (bind _boxcollision (Variables|/Game/Universal_Systems/Projectiles/BP_Projectile_Base.BP_Projectile_Base_C|GetBoxCollision _projectileref))
  (Audio|Components|Audio|Play (Variables|Default|GetWeapon_Audio) 0.0)
  (Variables|Default|SetownerToIgnoreAfterDrop (Variables|Default|GetowningCharacter))
  (bind _outhit (Collision|LineTraceByChannel _returnvalue_2 (+ _returnvalue_2 (* (Math|Vector|GetForwardVector _camerareference) 5e+03)) "TraceTypeQuery1" false 0 "None"))
  (Default|Trashball (Variables|Default|GetBPC_Attacks) (Math|Transform|MakeTransform _returnvalue (Math|Conversions|RotationFromXVector (Math|Vector|GetUnitDirection(Vector) _returnvalue (Math|Vector|SelectVector (.Location (Collision|BreakHitResult _outhit)) (.TraceEnd (Collision|BreakHitResult _outhit)) (.bBlockingHit (Collision|BreakHitResult _outhit))))) "1.000000,1.000000,1.000000") self "(R=1.000000,G=0.416298,B=0.000000,A=1.000000)" (Math|Float|MapRangeClamped attackPower 0.0 1.0 5e+02 4e+03) 0.75 0 (Utilities|Struct|MakeS_DamageInfo 25.0 "NewEnumerator2"))
  (Variables|Default|SetownerInCart (Variables|/Game/Characters/CharacterBase/BP_Character_Base.BP_Character_Base_C|GetisInCart (Variables|Default|GetowningCharacter))) ; Saves the cart status of \n'Owning Character' before \nthe ref is cleared.
  (Default|DropHeldWeapon (Variables|Default|GetowningCharacter))
  (if (not (Variables|Default|GetownerInCart))
    _
    (else
      (Collision|SetCollisionResponsetoChannel (Variables|Default|GetWeapon) "ECC_Vehicle" "ECR_Ignore")))
  (Collision|SetCollisionResponsetoChannel _boxcollision "ECC_PhysicsBody" "ECR_Ignore")
  (Class|PhysicsConstraintComponent|SetConstrainedComponents (Variables|Default|GetPC_PumpkinToProjectile) (Variables|Default|GetWeapon) "None" _boxcollision "None")
  (Variables|Default|SetisThrown true))

(event EventExplode
  (Utilities|FlowControl|DoOnce false
    (:Completed
      (Collision|SetCollisionResponsetoAllChannels (Variables|Default|GetWeapon) "ECR_Ignore")
      (bind _returnvalue (Game|SpawnActorfromClass "/Game/Weapons/PumpkinBomb/BP_PumpkinFracture.BP_PumpkinFracture_C" (Transformation|GetRelativeTransform (Variables|Default|GetWeapon)) "Undefined" "MultiplyWithRoot" 0 0))
      (Game|SpawnActorfromClass "/Engine/EditorResources/FieldNodes/FS_MasterField.FS_MasterField_C" (Math|Transform|MakeTransform (+ (.Location (Math|Transform|BreakTransform (Transformation|GetActorTransform _returnvalue))) "0.000000,-15.000000,0.000000") (.Rotation (Math|Transform|BreakTransform (Transformation|GetActorTransform _returnvalue))) (.Scale (Math|Transform|BreakTransform (Transformation|GetActorTransform _returnvalue)))) "Undefined" "MultiplyWithRoot" 0 0)
      (|CallParentFunction))))

(fn ConstructionScript
  (|CallParentFunction))