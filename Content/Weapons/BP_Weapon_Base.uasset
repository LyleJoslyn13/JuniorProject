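; Base weapon actor for melee, slingshot, bomb and umbrella types that characters pick up, holster, unholster and drop.
; Held weapons hang from the owner's physics constraints, placed at sockets chosen by weapon type, while holstering attaches them to sockets.
; In carts, it attaches the weapon and re-teleports it on a looping timer to stop shaking.
; It binds owner fire, aim and player camera dispatchers, leaving fire and aim handlers empty.
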(event Custom|Set%20position%20while%20in%20cart
  (bind _owningcharacter (Variables|Default|GetowningCharacter))
  (bind _weapontype (Variables|Default|GetweaponType))
  (bind _returnvalue (Utilities|Select :Index _weapontype :NewEnumerator3 "None" :NewEnumerator0 "inhand_slingshot" :NewEnumerator1 "inhand_racket" :NewEnumerator2 "inhand_bat" :NewEnumerator4 "back_equipment" :NewEnumerator5 "hand_equipment" :NewEnumerator6 "inhand_umbrella" :NewEnumerator7 "None"))
  (bind _mesh (Variables|/Script/Engine.Character|GetMesh _owningcharacter))
  (bind _returnvalue_2 (Transformation|GetSocketTransform _mesh _returnvalue "RTS_World"))
  (bind (_location _rotation) (Math|Transform|BreakTransform _returnvalue_2))
  (Transformation|SetWorldLocationAndRotation (Variables|Default|GetWeapon) _location _rotation false true))

(event Custom|Player%20Fire%20Weapon
  (params (attackTarget :type Actor%20Object%20Reference) (attackPower :type Float%20%28double-precision%29)))

(event Custom|NPC%20Fire%20Weapon
  (params (attackTarget :type Actor%20Object%20Reference) (attackPower :type Float%20%28double-precision%29)))

(event Custom|Character%20Animation%20Trigger%20Event)

(event Custom|updateCamera_Event
  (params (camera :type Camera%20Component%20Object%20Reference))
  (Variables|Default|SetcameraReference camera))

(event Custom|Character%20Animation%20Complete)

(event Custom|Update%20Personal%20Constraints)

(event Custom|On%20Update%20Aiming%20State
  (params (isAiming :type Boolean)))

(fn ConstructionScript)

(fn PlayWeaponSound
  (params (newSound :type Sound%20Base%20Object%20Reference))
  (bind _weapon_audio (Variables|Default|GetWeapon_Audio))
  (Audio|Components|Audio|SetSound _weapon_audio newSound)
  (Audio|Components|Audio|Play _weapon_audio 0.0))

(fn SetWeaponforCart
  (Transformation|AttachComponentToComponent (Variables|/Script/Engine.Character|GetMesh (Variables|Default|GetowningCharacter)) (Utilities|Select :Index (Variables|Default|GetweaponType) :NewEnumerator3 "None" :NewEnumerator0 "inhand_slingshot" :NewEnumerator1 "inhand_racket" :NewEnumerator2 "inhand_bat" :NewEnumerator4 "back_equipment" :NewEnumerator5 "hand_equipment" :NewEnumerator6 "inhand_umbrella" :NewEnumerator7 "None") "SnapToTarget" "SnapToTarget" "KeepWorld" true)
  (bind _returnvalue (Utilities|Time|SetTimerbyEvent (EventDispatchers|CreateEvent :!event Custom|Set%20position%20while%20in%20cart) 0.001 true true)) ; Stops weapons from shaking while in cart
  (Variables|Default|SetsetPositionInCartTimer _returnvalue)
  (Collision|SetCollisionResponsetoChannel (Variables|Default|GetWeapon) "ECC_Vehicle" "ECR_Ignore"))

(fn AttachArmor
  (params (armorPieceConstraint :type Physics%20Constraint%20Component%20Object%20Reference))
  (return false))

(fn DetachArmor
  (params (armorPiece :type BP%20Cart%20Armor%20Object%20Reference))
  (return false))

(fn Dropped
  (bind _weapon (Variables|Default|GetWeapon))
  (Utilities|Time|ClearandInvalidateTimerbyHandle (Variables|Default|GetsetPositionInCartTimer))
  (Components|SkinnedMesh|SetPhysicsAsset (Variables|Default|GetWeapon) (Variables|Default|GetweaponPhysicsAssetAsObject) true)
  (CallFunction|UpdatePersonalConstraints)
  (Physics|SetSimulatePhysics (Variables|Default|GetWeapon) true)
  (Class|PhysicsConstraintComponent|BreakConstraint (Utilities|Select :Index (Variables|Default|GetweaponType) :NewEnumerator3 0 :NewEnumerator0 (Variables|/Game/Characters/CharacterBase/BP_Character_Base.BP_Character_Base_C|GetPC_Hand_l (Variables|Default|GetowningCharacter)) :NewEnumerator1 (Variables|/Game/Characters/CharacterBase/BP_Character_Base.BP_Character_Base_C|GetPC_Hand_r (Variables|Default|GetowningCharacter)) :NewEnumerator2 (Variables|/Game/Characters/CharacterBase/BP_Character_Base.BP_Character_Base_C|GetPC_Hand_r (Variables|Default|GetowningCharacter)) :NewEnumerator4 (Variables|/Game/Characters/CharacterBase/BP_Character_Base.BP_Character_Base_C|GetPC_Back (Variables|Default|GetowningCharacter)) :NewEnumerator5 (Variables|/Game/Characters/CharacterBase/BP_Character_Base.BP_Character_Base_C|GetPC_Hand_r (Variables|Default|GetowningCharacter)) :NewEnumerator6 (Variables|/Game/Characters/CharacterBase/BP_Character_Base.BP_Character_Base_C|GetPC_Hand_r (Variables|Default|GetowningCharacter)) :NewEnumerator7 0))
  (Collision|SetCollisionProfileName _weapon "PhysicsActor" true :!class /Script/Engine.PrimitiveComponent)
  (Collision|SetCollisionResponsetoChannel _weapon "ECC_GameTraceChannel2" "ECR_Block")
  (EventDispatchers|UnbindallEventsfromFireWeapon (Variables|Default|GetowningCharacter))
  (EventDispatchers|UnbindEventfromUpdateCameraReference (Variables|Default|GetowningCharacter) (EventDispatchers|CreateEvent :!event Custom|updateCamera_Event)) ; (Don't use unbind all, it messes up cart camera \nafter picking up 3 slingshots)
  (EventDispatchers|UnbindallEventsfromSetAiming (Variables|Default|GetowningCharacter))
  (Transformation|DetachFromActor "KeepWorld" "KeepWorld" "KeepWorld")
  (Variables|Default|SetcameraReference 0)
  (Variables|Default|SetownerIsPlayer false)
  (Variables|Default|SetowningCharacter 0)
  (return true))

(fn GetWeaponType
  (return (Variables|Default|GetweaponType)))

(fn Holster
  (bind _owningcharacter (Variables|Default|GetowningCharacter))
  (bind _owningcharacter_2 (Variables|Default|GetowningCharacter))
  (bind _pc_hand_r (Variables|/Game/Characters/CharacterBase/BP_Character_Base.BP_Character_Base_C|GetPC_Hand_r _owningcharacter))
  (Utilities|Time|ClearandInvalidateTimerbyHandle (Variables|Default|GetsetPositionInCartTimer))
  (Class|PhysicsConstraintComponent|BreakConstraint (Utilities|Select :Index (Variables|Default|GetweaponType) :NewEnumerator3 0 :NewEnumerator0 (Variables|/Game/Characters/CharacterBase/BP_Character_Base.BP_Character_Base_C|GetPC_Hand_l _owningcharacter) :NewEnumerator1 _pc_hand_r :NewEnumerator2 _pc_hand_r :NewEnumerator4 0 :NewEnumerator5 _pc_hand_r :NewEnumerator6 _pc_hand_r :NewEnumerator7 0))
  (Physics|SetSimulatePhysics (Variables|Default|GetWeapon) false)
  (Collision|SetCollisionResponsetoAllChannels (Variables|Default|GetWeapon) "ECR_Ignore")
  (EventDispatchers|UnbindallEventsfromFireWeapon _owningcharacter_2)
  (EventDispatchers|UnbindallEventsfromSetAiming _owningcharacter_2)
  (bind _returnvalue (Transformation|AttachComponentToComponent (Variables|/Script/Engine.Character|GetMesh (Variables|Default|GetowningCharacter)) (Utilities|Select :Index (Variables|Default|GetweaponType) :NewEnumerator3 "None" :NewEnumerator0 "hip_holster_r" :NewEnumerator1 "back_holster_1" :NewEnumerator2 "back_holster_2" :NewEnumerator4 "back_equipment" :NewEnumerator5 "hand_equipment" :NewEnumerator6 "back_holster_3" :NewEnumerator7 "None") "SnapToTarget" "SnapToTarget" "KeepWorld" true))
  (return _returnvalue))

(fn Interactedwith
  (params (actorInitiatingInteraction :type BP%20Character%20Base%20Object%20Reference))
  (bind _output_get (Variables|Default|SetowningCharacter actorInitiatingInteraction))
  (Variables|Default|SetownerIsPlayer (Class|GameplayStatics|ObjectIsA _output_get "/Game/Characters/Player/Character/BP_Character_Player.BP_Character_Player_C")) ; This is imperative for when the\nplayer is in a cart and technically \nnot "controlled" anymore.
  (Components|SkinnedMesh|SetPhysicsAsset (Variables|Default|GetWeapon) (Variables|Default|GetweaponPhysicsAssetAsHeld) true)
  (CallFunction|UpdatePersonalConstraints)
  (Transformation|SetWorldLocationAndRotation (Variables|Default|GetWeapon) (.Location (Math|Transform|BreakTransform (Transformation|GetSocketTransform (Variables|/Script/Engine.Character|GetMesh (Variables|Default|GetowningCharacter)) (Utilities|Select :Index (Variables|Default|GetweaponType) :NewEnumerator3 "None" :NewEnumerator0 "inhand_slingshot" :NewEnumerator1 "inhand_racket" :NewEnumerator2 "inhand_bat" :NewEnumerator4 "back_equipment" :NewEnumerator5 "hand_equipment" :NewEnumerator6 "inhand_umbrella" :NewEnumerator7 "None") "RTS_World"))) (.Rotation (Math|Transform|BreakTransform (Transformation|GetSocketTransform (Variables|/Script/Engine.Character|GetMesh (Variables|Default|GetowningCharacter)) (Utilities|Select :Index (Variables|Default|GetweaponType) :NewEnumerator3 "None" :NewEnumerator0 "inhand_slingshot" :NewEnumerator1 "inhand_racket" :NewEnumerator2 "inhand_bat" :NewEnumerator4 "back_equipment" :NewEnumerator5 "hand_equipment" :NewEnumerator6 "inhand_umbrella" :NewEnumerator7 "None") "RTS_World"))) false true)
  (Class|PhysicsConstraintComponent|SetConstrainedComponents (Utilities|Select :Index (Variables|Default|GetweaponType) :NewEnumerator3 0 :NewEnumerator0 (Variables|/Game/Characters/CharacterBase/BP_Character_Base.BP_Character_Base_C|GetPC_Hand_l (Variables|Default|GetowningCharacter)) :NewEnumerator1 (Variables|/Game/Characters/CharacterBase/BP_Character_Base.BP_Character_Base_C|GetPC_Hand_r (Variables|Default|GetowningCharacter)) :NewEnumerator2 (Variables|/Game/Characters/CharacterBase/BP_Character_Base.BP_Character_Base_C|GetPC_Hand_r (Variables|Default|GetowningCharacter)) :NewEnumerator4 (Variables|/Game/Characters/CharacterBase/BP_Character_Base.BP_Character_Base_C|GetPC_Back (Variables|Default|GetowningCharacter)) :NewEnumerator5 (Variables|/Game/Characters/CharacterBase/BP_Character_Base.BP_Character_Base_C|GetPC_Hand_r (Variables|Default|GetowningCharacter)) :NewEnumerator6 (Variables|/Game/Characters/CharacterBase/BP_Character_Base.BP_Character_Base_C|GetPC_Hand_r (Variables|Default|GetowningCharacter)) :NewEnumerator7 0) (Variables|Default|GetWeapon) "" (Variables|/Script/Engine.Character|GetMesh (Variables|Default|GetowningCharacter)) (Utilities|Select :Index (Variables|Default|GetweaponType) :NewEnumerator3 "None" :NewEnumerator0 "hand_l" :NewEnumerator1 "hand_r" :NewEnumerator2 "hand_r" :NewEnumerator4 "spine_05" :NewEnumerator5 "hand_r" :NewEnumerator6 "hand_r" :NewEnumerator7 "None"))
  (Collision|SetCollisionResponsetoChannel (Variables|Default|GetWeapon) "ECC_GameTraceChannel2" "ECR_Ignore")
  (Variables|Default|SetcameraReference (Variables|/Game/Characters/CharacterBase/BP_Character_Base.BP_Character_Base_C|GetcameraReference (Variables|Default|GetowningCharacter)))
  (if (Variables|/Game/Characters/CharacterBase/BP_Character_Base.BP_Character_Base_C|GetisInCart (Variables|Default|GetowningCharacter))
    (CallFunction|SetWeaponforCart)
    (else
      (Utilities|Time|ClearandInvalidateTimerbyHandle (Variables|Default|GetsetPositionInCartTimer))))
  (if (Variables|Default|GetownerIsPlayer)
    (EventDispatchers|BindEventtoFireWeapon (Variables|Default|GetowningCharacter) (EventDispatchers|CreateEvent :!event Custom|Player%20Fire%20Weapon))
    (EventDispatchers|BindEventtoUpdateCameraReference (Variables|Default|GetowningCharacter) (EventDispatchers|CreateEvent :!event Custom|updateCamera_Event))
    (else
      (EventDispatchers|BindEventtoFireWeapon (Variables|Default|GetowningCharacter) (EventDispatchers|CreateEvent :!event Custom|NPC%20Fire%20Weapon))))
  (EventDispatchers|BindEventtoSetAiming (Variables|Default|GetowningCharacter) (EventDispatchers|CreateEvent :!event Custom|On%20Update%20Aiming%20State))
  (return true))

(fn IsHeldandSwinging
  (return (!= (Variables|Default|GetowningCharacter) 0) (Variables|Default|GetisSwinging)))

(fn Unholster
  (bind _weapon (Variables|Default|GetWeapon))
  (bind _owningcharacter (Variables|Default|GetowningCharacter))
  (bind _owningcharacter_2 (Variables|Default|GetowningCharacter))
  (bind _weapontype (Variables|Default|GetweaponType))
  (bind _returnvalue (Utilities|Select :Index _weapontype :NewEnumerator3 "None" :NewEnumerator0 "inhand_slingshot" :NewEnumerator1 "inhand_racket" :NewEnumerator2 "inhand_bat" :NewEnumerator4 "back_equipment" :NewEnumerator5 "hand_equipment" :NewEnumerator6 "inhand_umbrella" :NewEnumerator7 "None"))
  (bind _pc_hand_r (Variables|/Game/Characters/CharacterBase/BP_Character_Base.BP_Character_Base_C|GetPC_Hand_r _owningcharacter))
  (bind _mesh (Variables|/Script/Engine.Character|GetMesh _owningcharacter_2))
  (bind _returnvalue_2 (Transformation|GetSocketTransform _mesh _returnvalue "RTS_World"))
  (bind (_location _rotation) (Math|Transform|BreakTransform _returnvalue_2))
  (Transformation|DetachFromComponent (Variables|Default|GetWeapon) "KeepWorld" "KeepWorld" "KeepWorld" true)
  (Transformation|SetWorldLocationAndRotation (Variables|Default|GetWeapon) _location _rotation false true)
  (Class|PhysicsConstraintComponent|SetConstrainedComponents (Utilities|Select :Index (Variables|Default|GetweaponType) :NewEnumerator3 0 :NewEnumerator0 (Variables|/Game/Characters/CharacterBase/BP_Character_Base.BP_Character_Base_C|GetPC_Hand_l _owningcharacter) :NewEnumerator1 _pc_hand_r :NewEnumerator2 _pc_hand_r :NewEnumerator4 (Variables|/Game/Characters/CharacterBase/BP_Character_Base.BP_Character_Base_C|GetPC_Back _owningcharacter) :NewEnumerator5 _pc_hand_r :NewEnumerator6 _pc_hand_r :NewEnumerator7 0) (Variables|Default|GetWeapon) "" (Variables|/Script/Engine.Character|GetMesh (Variables|Default|GetowningCharacter)) (Utilities|Select :Index (Variables|Default|GetweaponType) :NewEnumerator3 "None" :NewEnumerator0 "hand_l" :NewEnumerator1 "hand_r" :NewEnumerator2 "hand_r" :NewEnumerator4 "spine_05" :NewEnumerator5 "hand_r" :NewEnumerator6 "hand_r" :NewEnumerator7 "None"))
  (Physics|SetSimulatePhysics _weapon true)
  (Collision|SetCollisionProfileName _weapon "PhysicsActor" true :!class /Script/Engine.PrimitiveComponent)
  (Collision|SetCollisionResponsetoChannel _weapon "ECC_Visibility" "ECR_Ignore")
  (if (Variables|/Game/Characters/CharacterBase/BP_Character_Base.BP_Character_Base_C|GetisInCart (Variables|Default|GetowningCharacter))
    (CallFunction|SetWeaponforCart)
    (else
      (Utilities|Time|ClearandInvalidateTimerbyHandle (Variables|Default|GetsetPositionInCartTimer))))
  (if (Variables|Default|GetownerIsPlayer)
    (EventDispatchers|BindEventtoFireWeapon (Variables|Default|GetowningCharacter) (EventDispatchers|CreateEvent :!event Custom|Player%20Fire%20Weapon))
    (EventDispatchers|BindEventtoUpdateCameraReference (Variables|Default|GetowningCharacter) (EventDispatchers|CreateEvent :!event Custom|updateCamera_Event))
    (EventDispatchers|BindEventtoSetAiming (Variables|Default|GetowningCharacter) (EventDispatchers|CreateEvent :!event Custom|On%20Update%20Aiming%20State))
    (return true)
    (else
      (EventDispatchers|BindEventtoFireWeapon (Variables|Default|GetowningCharacter) (EventDispatchers|CreateEvent :!event Custom|NPC%20Fire%20Weapon))
      (return true))))