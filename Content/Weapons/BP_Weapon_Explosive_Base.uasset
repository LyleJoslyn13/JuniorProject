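; Base explosive weapon that detonates once when fired by player or NPC, triggered by React, or on a death event.
; Its damage component takes velocity-scaled damage from hard impacts, and interaction activates effects and binds to the owner's death.
; Detonation sphere-traces unique actors, sending React for ignition or chain reactions and damaging characters.
; It then spawns particles, sound and a decal, fires a radial impulse and destroys itself.
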(event OnComponentHit(Weapon)
  (params (HitComponent :type Primitive%20Component%20Object%20Reference) (OtherActor :type Actor%20Object%20Reference) (OtherComp :type Primitive%20Component%20Object%20Reference) (NormalImpulse :type Vector :default "0, 0, 0") (Hit :type Hit%20Result%20Structure%20%28by%20ref%29))
  (bind (_bblockinghit _binitialoverlap _time _distance _location _impactpoint _normal _impactnormal _physmat _hitactor _hitcomponent) (Collision|BreakHitResult Hit))
  (bind _returnvalue (Transformation|GetComponentVelocity _hitcomponent))
  (bind _returnvalue_2 (Math|Vector|VectorLength _returnvalue))
  ;[1 1 1] Velocity Based Damage
  (if (>= (Math|Vector|VectorLength NormalImpulse) 8e+03)
    (if (!= OtherActor (Variables|Default|GetowningCharacter))
      (if (>= _returnvalue_2 2e+02)
        (CallFunction|TakeDamage (Utilities|Struct|MakeS_DamageInfo (/ _returnvalue_2 1e+01) "NewEnumerator1") 0 _hitactor)))))

(event Custom|Explode
  (bind _weapon (Variables|Default|GetWeapon))
  (bind _weapon_2 (Variables|Default|GetWeapon))
  (bind _weapon_3 (Variables|Default|GetWeapon))
  (bind _returnvalue (Transformation|GetWorldLocation _weapon))
  (bind _returnvalue_2 (Transformation|GetWorldLocation _weapon_3))
  (Utilities|FlowControl|DoOnce false
    (:Completed
      (Utilities|FlowControl|Sequence
        (:then_0
          (bind _outhits (Collision|MultiSphereTraceForObjects _returnvalue _returnvalue (Variables|Default|GetexplosionRadius) (Utilities|Array|MakeArray "ObjectTypeQuery4" "ObjectTypeQuery5" "ObjectTypeQuery6") false 0 "None"))
          (for _array_element _outhits
            (if (== (Utilities|Array|FindItem (Variables|Default|GethitActorsArray) (.HitActor (Collision|BreakHitResult _array_element))) -1)
              (Utilities|Array|AddUnique (Variables|Default|GethitActorsArray) (.HitActor (Collision|BreakHitResult _array_element)))
              (Class|BPIDestructible|React(Message) (.HitActor (Collision|BreakHitResult _array_element))) ; Ignite if Igniteable
              (if (Class|GameplayStatics|ObjectIsA (.HitActor (Collision|BreakHitResult _array_element)) "/Game/Characters/CharacterBase/BP_Character_Base.BP_Character_Base_C")
                (bind _asbp_character_base (Utilities|Casting|CastToBP_Character_Base (.HitActor (Collision|BreakHitResult _array_element))))
                (Default|TakeDamage _asbp_character_base (Utilities|Struct|MakeS_DamageInfo 1e+02 "NewEnumerator2" "NewEnumerator0" true) self (Variables|Default|GetWeapon))))))
        (:then_1
          (Effects|SpawnEmitteratLocation (Variables|Default|GetexplosionParticle) _returnvalue_2 "0, 0, 0" "2.000000,2.000000,2.000000") ; Explosion Particle
          (Audio|PlaySoundatLocation "/Game/Sounds/Explosion/BarrelBomb/Explosion_Cue.Explosion_Cue" _returnvalue_2 "0, 0, 0" 1.0 1.0 0.0 "/Game/Sounds/Explosion/SA_Explosions.SA_Explosions" 0 0 0) ; Explosion Sound
          (Class|RadialForceComponent|FireImpulse (Variables|Default|GetRadialForceExplosion))
          (Game|SpawnActorfromClass "/Game/Universal_Systems/Explosion/BP_Decal.BP_Decal_C" (Math|Transform|MakeTransform (Transformation|GetWorldLocation _weapon_2) (Math|Rotator|SelectRotator (Transformation|GetWorldRotation _weapon_2) "0, 0, 0" (Variables|Default|GetdecalShouldInheritRotation))) "Undefined" "MultiplyWithRoot" 0 (Variables|Default|GetdecalMaterial) 0)
          (Actor|DestroyActor))))))

(event Custom|On%20Death
  (CallFunction|Explode))

(event EventReact
  (bind _weapon (Variables|Default|GetWeapon))
  (bind _weapon_2 (Variables|Default|GetWeapon))
  (bind _weapon_3 (Variables|Default|GetWeapon))
  (bind _returnvalue (Transformation|GetWorldLocation _weapon))
  (bind _returnvalue_2 (Transformation|GetWorldLocation _weapon_3))
  (Utilities|FlowControl|DoOnce false
    (:Completed
      (Utilities|FlowControl|Sequence
        (:then_0
          (bind _outhits (Collision|MultiSphereTraceForObjects _returnvalue _returnvalue (Variables|Default|GetexplosionRadius) (Utilities|Array|MakeArray "ObjectTypeQuery4" "ObjectTypeQuery5" "ObjectTypeQuery6") false 0 "None"))
          (for _array_element _outhits
            (if (== (Utilities|Array|FindItem (Variables|Default|GethitActorsArray) (.HitActor (Collision|BreakHitResult _array_element))) -1)
              (Utilities|Array|AddUnique (Variables|Default|GethitActorsArray) (.HitActor (Collision|BreakHitResult _array_element)))
              (Class|BPIDestructible|React(Message) (.HitActor (Collision|BreakHitResult _array_element))) ; Ignite if Igniteable
              (if (Class|GameplayStatics|ObjectIsA (.HitActor (Collision|BreakHitResult _array_element)) "/Game/Characters/CharacterBase/BP_Character_Base.BP_Character_Base_C")
                (bind _asbp_character_base (Utilities|Casting|CastToBP_Character_Base (.HitActor (Collision|BreakHitResult _array_element))))
                (Default|TakeDamage _asbp_character_base (Utilities|Struct|MakeS_DamageInfo 1e+02 "NewEnumerator2" "NewEnumerator0" true) self (Variables|Default|GetWeapon))))))
        (:then_1
          (Effects|SpawnEmitteratLocation (Variables|Default|GetexplosionParticle) _returnvalue_2 "0, 0, 0" "2.000000,2.000000,2.000000") ; Explosion Particle
          (Audio|PlaySoundatLocation "/Game/Sounds/Explosion/BarrelBomb/Explosion_Cue.Explosion_Cue" _returnvalue_2 "0, 0, 0" 1.0 1.0 0.0 "/Game/Sounds/Explosion/SA_Explosions.SA_Explosions" 0 0 0) ; Explosion Sound
          (Class|RadialForceComponent|FireImpulse (Variables|Default|GetRadialForceExplosion))
          (Game|SpawnActorfromClass "/Game/Universal_Systems/Explosion/BP_Decal.BP_Decal_C" (Math|Transform|MakeTransform (Transformation|GetWorldLocation _weapon_2) (Math|Rotator|SelectRotator (Transformation|GetWorldRotation _weapon_2) "0, 0, 0" (Variables|Default|GetdecalShouldInheritRotation))) "Undefined" "MultiplyWithRoot" 0 (Variables|Default|GetdecalMaterial) 0)
          (Actor|DestroyActor))))))

(event EventPlayerFireWeapon
  (params (attackTarget :type Actor%20Object%20Reference) (attackPower :type Float%20%28double-precision%29))
  (CallFunction|Explode))

(event EventNPCFireWeapon
  (params (attackTarget :type Actor%20Object%20Reference) (attackPower :type Float%20%28double-precision%29))
  (CallFunction|Explode))

(event EventBeginPlay
  (Variables|/Script/Engine.RadialForceComponent|SetRadius (Variables|Default|GetRadialForceExplosion) (Variables|Default|GetexplosionRadius)))

(fn ConstructionScript
  (|CallParentFunction)
  (EventDispatchers|BindEventtoOnDeath (Variables|Default|GetBPC_DamageSystem) (EventDispatchers|CreateEvent :!event Custom|On%20Death)))

(fn Interactedwith
  (params (actorInitiatingInteraction :type BP%20Character%20Base%20Object%20Reference))
  (bind _successful (|CallParentFunction actorInitiatingInteraction))
  (Components|Activation|Activate (Variables|Default|GetPassive_Particle) false)
  (Audio|Components|Audio|Play (Variables|Default|GetWeapon_Audio) 0.0)
  (EventDispatchers|BindEventtoOnDeath (Variables|/Game/Characters/CharacterBase/BP_Character_Base.BP_Character_Base_C|GetBPC_DamageSystem (Variables|Default|GetowningCharacter)) (EventDispatchers|CreateEvent :!event Custom|Explode))
  (return _successful))

(fn GetCurrentHealth
  (return 0.0))

(fn GetMaxHealth
  (return 0.0))

(fn GetTeamNumber
  (return 0))

(fn Heal
  (params (AmountToHeal :type Float%20%28double-precision%29))
  (return 0.0))

(fn IsAttacking
  (return false))

(fn IsDead
  (return (Variables|/Game/Universal_Systems/DamageSystem/BPC_DamageSystem.BPC_DamageSystem_C|GetIsDead (Variables|Default|GetBPC_DamageSystem))))

(fn ReserveAttackToken
  (params (Amount :type Integer))
  (return false))

(fn TakeDamage
  (params (Damageinfo :type S%20Damage%20Info%20Structure) (DamageCausingActor :type Actor%20Object%20Reference) (DamageCausingComponent :type Object%20Object%20Reference))
  (bind _wasdamaged (Default|TakeDamage (Variables|Default|GetBPC_DamageSystem) Damageinfo DamageCausingActor))
  (return _wasdamaged))