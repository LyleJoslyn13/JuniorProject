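; Base Blueprint for two-handed weapons that attaches the weapon to the owning character's left hand while aiming.
; While aiming, a looping timer polls whether the offhand detector overlaps the character mesh close to the LHand socket.
; On a match, a physics constraint binds the weapon to that hand and polling stops.
; Ending aim, holstering or dropping breaks the constraint; unholstering or interacting restarts polling if aiming.
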(event Custom|Check%20for%20OffHand
  ;[1 1 1] Constrain to Left Hand when near
  (if (and (Class|PrimitiveComponent|IsOverlappingComponent (Variables|Default|GetleftHandOverlapDetector) (Variables|/Script/Engine.Character|GetMesh (Variables|Default|GetowningCharacter))) (<= (Math|Vector|Distance(Vector) (Transformation|GetWorldLocation (Variables|Default|GetleftHandOverlapDetector)) (Transformation|GetSocketLocation (Variables|/Script/Engine.Character|GetMesh (Variables|Default|GetowningCharacter)) "LHand")) 15.0))
    (Class|PhysicsConstraintComponent|SetConstrainedComponents (Variables|Default|GetPC_GuideConstraintSphereToHand) (Variables|Default|GetWeapon) "None" (Variables|/Script/Engine.Character|GetMesh (Variables|Default|GetowningCharacter)) "LHand")
    (Utilities|Time|ClearandInvalidateTimerbyHandle (Variables|Default|GetcheckForOffhandTimer))))

(event Custom|Break%20Left%20Hand%20And%20Timer
  ;[1 1 1] Constrain to Left Hand when near
  (Class|PhysicsConstraintComponent|BreakConstraint (Variables|Default|GetPC_GuideConstraintSphereToHand))
  (Utilities|Time|ClearandInvalidateTimerbyHandle (Variables|Default|GetcheckForOffhandTimer)))

(event Custom|Start%20Offhand%20Timer
  ;[1 1 1] Constrain to Left Hand when near
  (bind _returnvalue (Utilities|Time|SetTimerbyEvent (EventDispatchers|CreateEvent :!event Custom|Check%20for%20OffHand) 0.1 true))
  (Variables|Default|SetcheckForOffhandTimer _returnvalue))

(event EventOnUpdateAimingState
  (params (isAiming :type Boolean))
  ;[1 1 1] Constrain to Left Hand when near
  ;;[1 1 1] On Aim Update
  (if isAiming
    (CallFunction|StartOffhandTimer)
    (else
      (CallFunction|BreakLeftHandandTimer))))

(fn ConstructionScript
  (|CallParentFunction))

(fn Holster
  (CallFunction|BreakLeftHandandTimer)
  (bind _successful (|CallParentFunction))
  (return _successful))

(fn Unholster
  (bind _successful (|CallParentFunction))
  (if (Variables|/Game/Characters/CharacterBase/BP_Character_Base.BP_Character_Base_C|GetisAiming (Variables|Default|GetowningCharacter))
    (CallFunction|StartOffhandTimer))
  (return _successful))

(fn Dropped
  (CallFunction|BreakLeftHandandTimer)
  (bind _successful (|CallParentFunction))
  (return _successful))

(fn Interactedwith
  (params (actorInitiatingInteraction :type BP%20Character%20Base%20Object%20Reference))
  (bind _successful (|CallParentFunction actorInitiatingInteraction))
  (if (Variables|/Game/Characters/CharacterBase/BP_Character_Base.BP_Character_Base_C|GetisAiming (Variables|Default|GetowningCharacter))
    (CallFunction|StartOffhandTimer))
  (return _successful))