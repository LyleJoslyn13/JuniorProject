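; Two-handed baseball bat weapon that plays grip and swing sounds and tracks whether the character is mid-swing.
; Firing sets the swing flag and weapon state, and animation completion clears the flag.
; Pickup and unholster bind to the owner's animation attach notify and disable impact overlaps while in a cart; drop and holster unbind.
; The impact collider's object-hit sound logic is disconnected, so overlaps currently play nothing.
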(event OnComponentBeginOverlap(CollisionForImpactSound)
  (params (OverlappedComponent :type Primitive%20Component%20Object%20Reference) (OtherActor :type Actor%20Object%20Reference) (OtherComp :type Primitive%20Component%20Object%20Reference) (OtherBodyIndex :type Integer) (bFromSweep :type Boolean) (SweepResult :type Hit%20Result%20Structure%20%28by%20ref%29)))

(event Custom|Bat%20Pulled%20Back
  (CallFunction|PlayWeaponSound "/Game/Sounds/BaseballBat/TightenGrip/BatGripTighten_Cue.BatGripTighten_Cue"))

(event EventCharacterAnimationComplete
  (Variables|Default|SetisSwinging false))

(event EventPlayerFireWeapon
  (params (attackTarget :type Actor%20Object%20Reference) (attackPower :type Float%20%28double-precision%29))
  (Variables|Default|SetisSwinging true)
  (Variables|Default|SetweaponStates "NewEnumerator0")
  (CallFunction|PlayWeaponSound "/Game/Sounds/BaseballBat/Swing/BatSwingWoosh_Cue.BatSwingWoosh_Cue"))

(fn ConstructionScript
  (|CallParentFunction))

(fn Dropped
  (EventDispatchers|UnbindEventfromAnimationNotifyAttach (Variables|/Game/Characters/CharacterBase/BP_Character_Base.BP_Character_Base_C|GetanimationBP_Ref (Variables|Default|GetowningCharacter)) (EventDispatchers|CreateEvent :!event Custom|Bat%20Pulled%20Back))
  (Collision|SetCollisionEnabled (Variables|Default|GetCollisionForImpactSound) "QueryOnly")
  (bind _successful (|CallParentFunction))
  (return _successful))

(fn Holster
  (EventDispatchers|UnbindEventfromAnimationNotifyAttach (Variables|/Game/Characters/CharacterBase/BP_Character_Base.BP_Character_Base_C|GetanimationBP_Ref (Variables|Default|GetowningCharacter)) (EventDispatchers|CreateEvent :!event Custom|Bat%20Pulled%20Back))
  (Collision|SetCollisionEnabled (Variables|Default|GetCollisionForImpactSound) "NoCollision")
  (bind _successful (|CallParentFunction))
  (return _successful))

(fn Unholster
  (bind _successful (|CallParentFunction))
  (EventDispatchers|BindEventtoAnimationNotifyAttach (Variables|/Game/Characters/CharacterBase/BP_Character_Base.BP_Character_Base_C|GetanimationBP_Ref (Variables|Default|GetowningCharacter)) (EventDispatchers|CreateEvent :!event Custom|Bat%20Pulled%20Back))
  (Collision|SetCollisionEnabled (Variables|Default|GetCollisionForImpactSound) "QueryOnly")
  (Variables|/Script/Engine.PrimitiveComponent|SetbGenerateOverlapEvents (Variables|Default|GetCollisionForImpactSound) (not (Variables|/Game/Characters/CharacterBase/BP_Character_Base.BP_Character_Base_C|GetisInCart (Variables|Default|GetowningCharacter)))) ; (Keeps triggering sounds while in cart, this\nfixes it, could make detection for play in carts\nweapon and block that instead)
  (return _successful))

(fn Interactedwith
  (params (actorInitiatingInteraction :type BP%20Character%20Base%20Object%20Reference))
  (bind _successful (|CallParentFunction actorInitiatingInteraction))
  (EventDispatchers|BindEventtoAnimationNotifyAttach (Variables|/Game/Characters/CharacterBase/BP_Character_Base.BP_Character_Base_C|GetanimationBP_Ref (Variables|Default|GetowningCharacter)) (EventDispatchers|CreateEvent :!event Custom|Bat%20Pulled%20Back))
  (Variables|/Script/Engine.PrimitiveComponent|SetbGenerateOverlapEvents (Variables|Default|GetCollisionForImpactSound) (not (Variables|/Game/Characters/CharacterBase/BP_Character_Base.BP_Character_Base_C|GetisInCart (Variables|Default|GetowningCharacter)))) ; (Keeps triggering sounds while in cart, this\nfixes it, could make detection for play in carts\nweapon and block that instead)
  (return _successful))