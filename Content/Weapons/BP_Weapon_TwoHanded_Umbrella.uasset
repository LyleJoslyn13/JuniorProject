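; Two-handed umbrella weapon that the player opens and closes with the fire input.
; Firing toggles the open state, swapping visibility between the closed and open cover components.
; The open cover gains physics-actor collision that ignores visibility, camera, static world and vehicle channels, and loses all collision when closed.
; Holster calls UpdatePersonalConstraints, which forces the umbrella closed, before running the parent holster logic.
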(event EventPlayerFireWeapon
  (params (attackTarget :type Actor%20Object%20Reference) (attackPower :type Float%20%28double-precision%29))
  (bind _umbrellacoverclosed (Variables|Default|GetUmbrellaCoverCLOSED))
  (bind _umbrellacoveropen (Variables|Default|GetUmbrellaCoverOPEN))
  (if (not (Variables|Default|GetumbrellaOpen))
    (Variables|Default|SetumbrellaOpen true)
    (Rendering|SetVisibility _umbrellacoverclosed false false)
    (Rendering|SetVisibility _umbrellacoveropen true false)
    (Collision|SetCollisionProfileName _umbrellacoveropen "PhysicsActor" true :!class /Script/Engine.PrimitiveComponent)
    (Collision|SetCollisionResponsetoChannel _umbrellacoveropen "ECC_Visibility" "ECR_Ignore")
    (Collision|SetCollisionResponsetoChannel _umbrellacoveropen "ECC_Camera" "ECR_Ignore")
    (Collision|SetCollisionResponsetoChannel _umbrellacoveropen "ECC_WorldStatic" "ECR_Ignore")
    (Collision|SetCollisionResponsetoChannel _umbrellacoveropen "ECC_Vehicle" "ECR_Ignore")
    (else
      (Variables|Default|SetumbrellaOpen false)
      (Rendering|SetVisibility _umbrellacoverclosed true false)
      (Rendering|SetVisibility _umbrellacoveropen false false)
      (Collision|SetCollisionProfileName _umbrellacoveropen "NoCollision" true :!class /Script/Engine.PrimitiveComponent))))

(event EventUpdatePersonalConstraints
  (bind _umbrellacoveropen (Variables|Default|GetUmbrellaCoverOPEN))
  (Variables|Default|SetumbrellaOpen false)
  (Rendering|SetVisibility (Variables|Default|GetUmbrellaCoverCLOSED) true false)
  (Rendering|SetVisibility _umbrellacoveropen false false)
  (Collision|SetCollisionProfileName _umbrellacoveropen "NoCollision" true :!class /Script/Engine.PrimitiveComponent))

(fn ConstructionScript
  (|CallParentFunction))

(fn Holster
  (CallFunction|UpdatePersonalConstraints)
  (bind _successful (|CallParentFunction))
  (return _successful))