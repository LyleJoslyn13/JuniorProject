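; Bomb boost cart attachment that rockets its owner forward, then becomes an explosive once detached.
; On BeginPlay it adds a physics thruster to the owner, easing thrust after a brief burst, and starts a looping timer, likely for nearby-object capsule traces that send hit reactions.
; Detaching swaps the owner's thruster for a weak one on itself.
; It explodes on hitting an enemy or after a delay, lingering briefly for effects.
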(event Custom|Check%20For%20Nearby%20Objects
  (bind _weapon (Variables|Default|GetWeapon))
  (bind _returnvalue (Transformation|GetSocketLocation _weapon "Particle"))
  (bind _outhit (Class|KismetSystemLibrary|CapsuleTraceSingleforObjects _returnvalue (+ _returnvalue (* (Math|Vector|GetUpVector (Variables|Default|GetWeapon)) -1.5e+02)) 5e+01 1e+01 (Utilities|Array|MakeArray "ObjectTypeQuery4") false 0 "None" true))
  (Class|BPIDestructible|React(Message) (.HitActor (Collision|BreakHitResult _outhit)) true)
  (if (and (Variables|Default|Getdetached) (Class|GameplayStatics|ObjectIsA (.HitActor (Collision|BreakHitResult _outhit)) "/Game/Characters/Enemy/BP_Character_Enemy.BP_Character_Enemy_C"))
    (Utilities|FlowControl|DoOnce false
      (:Completed
        (CallFunction|Explode)))))

(event Custom|Explode
  (Utilities|FlowControl|DoOnce false
    (:Completed
      (Utilities|Time|ClearandInvalidateTimerbyHandle (Variables|Default|GetnearbyObjectTimer))
      (Game|SpawnActorfromClass "/Game/Universal_Systems/BP_Explosion.BP_Explosion_C" (Transformation|GetActorTransform) "Undefined" "MultiplyWithRoot" 0 1e+02 3e+02 5e+04 "/Game/StarterContent/Particles/P_Explosion.P_Explosion" "/Game/Sounds/Explosion/BombBoost/Explosion_BombBoost_Cue.Explosion_BombBoost_Cue" "/Game/Universal_Systems/Explosion/M_ScortchMark.M_ScortchMark" false true 0)
      ;[0.005208 0.005208 0.005208 0.495] (Lets particle and sound effects finish before completely destroying actor)
      (Components|DestroyComponent (Variables|Default|GetWeapon))
      (Utilities|FlowControl|Delay 3.0)
      (Actor|DestroyActor))))

(event Custom|Start%20Bomb%20Boost
  (Utilities|FlowControl|Sequence
    (:then_0
      (bind _returnvalue (AddComponent|AddPhysicsThrusterComponent (Components|GetOwner) false (Math|Transform|MakeTransform "0, 0, 0")))
      (Variables|/Script/Engine.PhysicsThrusterComponent|SetThrustStrength _returnvalue -3e+05)
      (Components|Activation|Activate _returnvalue false)
      (Variables|Default|SetthrusterComponent _returnvalue)
      (Utilities|FlowControl|Delay 0.5)
      (Variables|/Script/Engine.PhysicsThrusterComponent|SetThrustStrength _returnvalue -2e+05))
    (:then_1
      (bind _returnvalue_2 (Utilities|Time|SetTimerbyEvent (EventDispatchers|CreateEvent :!event Custom|Check%20For%20Nearby%20Objects) 0.1 true))
      (Variables|Default|SetnearbyObjectTimer _returnvalue_2))))

(event EventBeginPlay
  (CallFunction|StartBombBoost))

(event EventOnDetach
  (bind _thrustercomponent (Variables|Default|GetthrusterComponent))
  (Variables|Default|Setdetached true)
  (bind _returnvalue (AddComponent|AddPhysicsThrusterComponent false (Math|Transform|MakeTransform "0, 0, 0" "-90.000000,0.000000,0.000000")))
  (Variables|/Script/Engine.PhysicsThrusterComponent|SetThrustStrength _returnvalue 1.0)
  (Components|Activation|Activate _returnvalue false)
  ;[1 1 1] Remove Owner's Thruster
  (Components|Activation|Deactivate _thrustercomponent)
  (Components|DestroyComponent _thrustercomponent)
  (Utilities|FlowControl|Delay 3.0)
  (Components|Activation|Deactivate (Variables|Default|GetNE_ParticleEffect))
  (Components|DestroyComponent _returnvalue)
  (Audio|Components|Audio|FadeOut (Variables|Default|GetSpeaker) 1.0 0.0 "Linear" :!class /Script/Engine.AudioComponent)
  (CallFunction|Explode))

(fn ConstructionScript
  (|CallParentFunction))