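; Cart weapon attachment actor that sets its mesh by weapon type, with most logic serving the Bomb Boost gas canister.
; Bomb Boost adds a physics thruster to the owning cart, plays fire and sound effects, and runs timed capsule traces sending React messages to hit physics bodies.
; On detach, Plow and Turret fade away, while Bomb Boost swaps the cart's thruster for its own, then explodes after a delay.
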(event Custom|Check%20For%20Nearby%20Objects
  (bind _staticmesh (Variables|Default|GetStaticMesh))
  (bind _returnvalue (Transformation|GetSocketLocation _staticmesh "Particle"))
  (bind _outhit (Class|KismetSystemLibrary|CapsuleTraceSingleforObjects _returnvalue (+ _returnvalue (* (Math|Vector|GetUpVector (Variables|Default|GetStaticMesh)) -1.5e+02)) 5e+01 1e+01 (Utilities|Array|MakeArray "ObjectTypeQuery4") false 0 "None" true))
  (Class|BPIDestructible|React(Message) (.HitActor (Collision|BreakHitResult _outhit)) true)
  (if (and (Variables|Default|Getdetached) (Class|GameplayStatics|ObjectIsA (.HitActor (Collision|BreakHitResult _outhit)) "/Game/Characters/Enemy/BP_Character_Enemy.BP_Character_Enemy_C"))
    (Utilities|FlowControl|DoOnce false)))

(event Custom|On%20Detach
  (bind _thrustercomponent (Variables|Default|GetthrusterComponent))
  (Variables|Default|Setdetached true)
  (switch Utilities|FlowControl|Switch|SwitchonE_CartWeapons (Variables|Default|GetcartWeapon)
    (:NewEnumerator1
      (Default|FadeAwayActor (Variables|Default|GetBP_FadeAway) (Variables|Default|GetStaticMesh) 5.0 :!label _label))
    (:NewEnumerator2
      (goto _label))
    (:NewEnumerator4
      (bind _returnvalue (AddComponent|AddPhysicsThrusterComponent false (Math|Transform|MakeTransform "0, 0, 0" "-90.000000,0.000000,0.000000")))
      (Variables|/Script/Engine.PhysicsThrusterComponent|SetThrustStrength _returnvalue 1.0)
      (Components|Activation|Activate _returnvalue false)
      ;[1 1 1] Remove Owner's Thruster
      (Components|Activation|Deactivate _thrustercomponent)
      (Components|DestroyComponent _thrustercomponent)
      (Utilities|FlowControl|Delay 3.0)
      (Components|Activation|Deactivate (Variables|Default|GetNE_ParticleEffect))
      (Utilities|Time|ClearandInvalidateTimerbyHandle (Variables|Default|GetnearbyObjectTimer))
      (Components|DestroyComponent _returnvalue)
      (Audio|Components|Audio|FadeOut (Variables|Default|GetSpeaker) 1.0 0.0 "Linear" :!class /Script/Engine.AudioComponent)
      (CallFunction|Explode))))

(event Custom|Explode
  (Game|SpawnActorfromClass "/Game/Universal_Systems/BP_Explosion.BP_Explosion_C" (Transformation|GetActorTransform) "Undefined" "MultiplyWithRoot" 0 1e+02 3e+02 5e+04 "/Game/StarterContent/Particles/P_Explosion.P_Explosion" "/Game/Sounds/Explosion/BombBoost/Explosion_BombBoost_Cue.Explosion_BombBoost_Cue" "/Game/Universal_Systems/Explosion/M_ScortchMark.M_ScortchMark" false true 0)
  ;[0.005208 0.005208 0.005208 0.495] (Lets particle and sound effects finish before completely destroying actor)
  (Components|DestroyComponent (Variables|Default|GetStaticMesh))
  (Utilities|FlowControl|Delay 3.0)
  (Actor|DestroyActor))

(event Custom|Start%20Bomb%20Boost
  (bind _speaker (Variables|Default|GetSpeaker))
  (Utilities|FlowControl|Sequence
    (:then_0
      (bind _returnvalue (AddComponent|AddPhysicsThrusterComponent (Components|GetOwner) false (Math|Transform|MakeTransform "0, 0, 0")))
      (Variables|/Script/Engine.PhysicsThrusterComponent|SetThrustStrength _returnvalue -3e+05)
      (Components|Activation|Activate _returnvalue false)
      (Variables|Default|SetthrusterComponent _returnvalue)
      (Utilities|FlowControl|Delay 0.5)
      (Variables|/Script/Engine.PhysicsThrusterComponent|SetThrustStrength _returnvalue -2e+05))
    (:then_1
      (Class|NiagaraComponent|SetAsset (Variables|Default|GetNE_ParticleEffect) "/Game/Characters/Player/Cart/Attachments/BombBoost/NE_FireTrail_System.NE_FireTrail_System" true)
      (Transformation|SetWorldLocation (Variables|Default|GetNE_ParticleEffect) (Transformation|GetSocketLocation (Variables|Default|GetStaticMesh) "Particle") false true)
      (Components|Activation|Activate (Variables|Default|GetNE_ParticleEffect) false)
      (Audio|Components|Audio|SetSound _speaker "/Game/Sounds/Thruster/Thruster_Cue.Thruster_Cue")
      (Audio|Components|Audio|Play _speaker 0.0)
      (bind _returnvalue_2 (Utilities|Time|SetTimerbyEvent (EventDispatchers|CreateEvent :!event Custom|Check%20For%20Nearby%20Objects) 0.1 true))
      (Variables|Default|SetnearbyObjectTimer _returnvalue_2))))

(fn ConstructionScript)

(fn SetAttachment
  (params (cartWeapon :type E_CartWeapons%20Enum :default "NewEnumerator0"))
  (bind _output_get (Variables|Default|SetcartWeapon cartWeapon))
  (Components|StaticMesh|SetStaticMesh (Variables|Default|GetStaticMesh) (Utilities|Select :Index _output_get :NewEnumerator0 "/PCG/SampleContent/MeshSockets/Meshes/1M_CubeWithSocket.1M_CubeWithSocket" :NewEnumerator1 "/Game/Characters/Player/Cart/Attachments/Plow/diggerbucket.diggerbucket" :NewEnumerator2 0 :NewEnumerator4 "/Game/Characters/Player/Cart/Attachments/BombBoost/gas_canister.gas_canister" :NewEnumerator6 0))
  (Utilities|FlowControl|Sequence
    (:then_0
      (switch Utilities|FlowControl|Switch|SwitchonE_CartWeapons (Variables|Default|GetcartWeapon)
        (:NewEnumerator4
          (Class|PrimitiveComponent|SetMassOverrideinKg (Variables|Default|GetStaticMesh) "None" 0.0 true)
          (CallFunction|StartBombBoost))))
    (:then_1
      (return (Variables|Default|GetStaticMesh)))))