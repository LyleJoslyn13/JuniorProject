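; BP_CartArmor is a metal armor plate attachment for the player's cart that breaks off when shot.
; On BeginPlay it picks a front or side sheet mesh from IsSmallArmor and gives its paint a random color through a dynamic material instance.
; The first projectile hit tells the owner to detach it, switches its collision and starts a delayed fade-out.
; Its health, team and damage functions are stubs returning zero or false.
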(event EventBeginPlay
  (bind _armor (Variables|Default|GetArmor))
  ;[0.2656 0.2656 0.2656] Sets armor piece mesh
  (Components|StaticMesh|SetStaticMesh (Variables|Default|GetArmor) (select (Variables|Default|GetisSmallArmor) "/Game/Characters/Player/Cart/ShoppingCart/NewCart/Cart_mesh_Car_FrontMetalSheet.Cart_mesh_Car_FrontMetalSheet" "/Game/Characters/Player/Cart/ShoppingCart/NewCart/Cart_mesh_Car_SideMetalSheet.Cart_mesh_Car_SideMetalSheet"))
  ;[1 0 0.5914] Assigns random color to paint
  (bind _returnvalue (Rendering|Material|CreateDynamicMaterialInstance _armor 0 (Rendering|Material|GetMaterial _armor 0) "None" :!class /Script/Engine.PrimitiveComponent))
  (Rendering|Material|SetVectorParameterValue _returnvalue "Paint" (Math|Color|MakeColor (Math|Random|RandomFloat) (Math|Random|RandomFloatinRange 0.15 1.0) (Math|Random|RandomFloatinRange 0.0 0.75)) :!class /Script/Engine.MaterialInstanceDynamic))

(event Collision|EventHit
  (params (MyComp :type Primitive%20Component%20Object%20Reference) (Other :type Actor%20Object%20Reference) (OtherComp :type Primitive%20Component%20Object%20Reference) (bSelfMoved :type Boolean) (HitLocation :type Vector :default "0, 0, 0") (HitNormal :type Vector :default "0, 0, 0") (NormalImpulse :type Vector :default "0, 0, 0") (Hit :type Hit%20Result%20Structure%20%28by%20ref%29))
  ;[1 0.7963 0.08854] Detach if shot
  (if (Class|GameplayStatics|ObjectIsA Other "/Game/Universal_Systems/Projectiles/BP_Projectile_Base.BP_Projectile_Base_C")
    (Utilities|FlowControl|DoOnce false
      (:Completed
        (Class|BPIInteractive|DetachArmor(Message) (Components|GetOwner) self)
        (Collision|SetCollisionResponsetoChannel (Variables|Default|GetArmor) "ECC_WorldStatic" "ECR_Block")
        (Collision|SetCollisionResponsetoChannel (Variables|Default|GetArmor) "ECC_Vehicle" "ECR_Ignore")
        (Default|FadeAwayComponent (Variables|Default|GetBP_FadeAway) (Variables|Default|GetArmor) 5.0)))))

(fn ConstructionScript)

(fn GetCurrentHealth
  (return 0.0))

(fn GetMaxHealth
  (return 0.0))

(fn GetTeamNumber
  (return 0))

(fn Heal
  (params (AmountToHeal :type Float%20%28double-precision%29))
  (return 0.0))

(fn IsAttacking
  (return false))

(fn IsDead
  (return false))

(fn ReserveAttackToken
  (params (Amount :type Integer))
  (return false))

(fn TakeDamage
  (params (Damageinfo :type S%20Damage%20Info%20Structure) (DamageCausingActor :type Actor%20Object%20Reference) (DamageCausingComponent :type Object%20Object%20Reference))
  (return false))