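; Auto-targeting turret attachment for the player cart that shoots at nearby living enemies.
; Looping timers drive a sphere-trace scan for the closest enemy and smooth neck aiming; acquiring a target starts a firing timer and changes the light color.
; Bullets head straight at the enemy regardless of barrel alignment, unless a trace hits the owning cart.
; Fire effects precede timed detachment, which stops the timers and drops the parts as physics debris.
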(event Custom|Aim%20At%20Target
  (bind _activetarget (Variables|Default|GetactiveTarget))
  (bind _turretneck (Variables|Default|GetturretNeck))
  (bind _turretneck_2 (Variables|Default|GetturretNeck))
  (bind _returnvalue (Transformation|GetWorldLocation _turretneck_2))
  (bind _mesh (Variables|/Script/Engine.Character|GetMesh _activetarget))
  (bind _returnvalue_2 (Transformation|GetSocketLocation _mesh "spine_04"))
  (bind _returnvalue_3 (Math|Rotator|FindLookatRotation _returnvalue _returnvalue_2))
  (bind (_roll _pitch _yaw) (Math|Rotator|BreakRotator _returnvalue_3))
  ;[0.004252 0 1] Aim
  (if (Variables|Default|GethasTarget)
    (Transformation|SetWorldRotation (Variables|Default|GetturretNeck) (Math|Interpolation|RInterpTo (Transformation|GetWorldRotation (Variables|Default|GetturretNeck)) (Math|Rotator|MakeRotator _roll _pitch _yaw) (Utilities|Time|GetWorldDeltaSeconds) 4e+01) false false)
    (else
      (Transformation|SetRelativeRotation _turretneck (Math|Interpolation|RInterpTo (Variables|/Script/Engine.SceneComponent|GetRelativeRotation _turretneck) "0, 0, 0" (Utilities|Time|GetWorldDeltaSeconds) 5.0) false false))))

(event Custom|Sense%20Nearby%20Targets
  (bind _turrethead (Variables|Default|GetturretHead))
  (bind _returnvalue (Transformation|GetWorldLocation _turrethead))
  ;[0.476 1 0] Scan for Nearby Targets
  (bind _outhits (Collision|MultiSphereTraceForObjects _returnvalue _returnvalue (Variables|Default|GetattackRange) (Utilities|Array|MakeArray "ObjectTypeQuery3") false (Utilities|Array|MakeArray (Components|GetOwner) (select (Variables|Default|GetownedByCart) (Variables|/Game/Characters/Player/Cart/ShoppingCartPawn/BP_PlayerCart.BP_PlayerCart_C|GetrefToCharacterInCart (Variables|Default|GetowningCart)) 0)) "None"))
  (for _array_element _outhits
    (if (Class|GameplayStatics|ObjectIsA (.HitActor (Collision|BreakHitResult _array_element)) "/Game/Characters/Enemy/BP_Character_Enemy.BP_Character_Enemy_C")
      (bind _dead (Class|BPIDamagable|IsDead(Message) (.HitActor (Collision|BreakHitResult _array_element))))
      (if (not _dead)
        (Utilities|Array|AddUnique (Variables|Default|GetnearbyTargets) (.HitActor (Collision|BreakHitResult _array_element)))
        (if (< (Math|Vector|Distance(Vector) (Transformation|GetActorLocation (.HitActor (Collision|BreakHitResult _array_element))) (Transformation|GetActorLocation)) (Variables|Default|GetshortestDistanceToNearbyTarget)) ; Set new actor if it's closer \nthan the previous one
          (Variables|Default|SetshortestDistanceToNearbyTarget (Math|Vector|Distance(Vector) (Transformation|GetActorLocation (.HitActor (Collision|BreakHitResult _array_element))) (Transformation|GetActorLocation)))
          (Variables|Default|SetclosestEnemy (.HitActor (Collision|BreakHitResult _array_element)))))))
  (if (== (Utilities|Array|Length (Variables|Default|GetnearbyTargets)) 0) ; Are there NO nearby targets?
    (Utilities|FlowControl|DoOnce false :!label _label
      (:Completed
        (CallFunction|NoTarget)
        (Utilities|Array|Clear (Variables|Default|GetnearbyTargets))
        (Development|PrintString "NO TARGETS" true true "(R=1.000000,G=0.000000,B=0.036510,A=1.000000)")))
    (else
      (Utilities|FlowControl|Sequence
        (:then_0
          (goto _label Reset))
        (:then_1
          (Utilities|Array|Clear (Variables|Default|GetnearbyTargets))
          (if (== (Variables|Default|GetclosestEnemy) (Variables|Default|GetactiveTarget)) ; Is the closest enemy the active target?
            (Development|PrintString "Closest Enemy IS Active Target" true true "(R=1.000000,G=0.898733,B=0.000000,A=1.000000)")
            (Variables|Default|SetshortestDistanceToNearbyTarget 99999.0) ; Sets default distance to greater value than necessary, \nso the first item in array will always have it's distance \nbecome the one to compare the rest to
            (else
              (CallFunction|TargetAcquired))))))))

(event Custom|No%20Target
  (Variables|Default|SethasTarget false)
  (Variables|Default|SetclosestEnemy 0)
  (Variables|Default|SetactiveTarget 0)
  (Variables|Default|SetshortestDistanceToNearbyTarget 99999.0) ; Sets default distance to greater value than necessary, \nso the first item in array will always have it's distance \nbecome the one to compare the rest to
  (Utilities|Time|ClearandInvalidateTimerbyHandle (Variables|Default|GetfireTimer))
  (Rendering|Components|Light|SetLightColor (Variables|Default|GetPointLight) "(R=1.000000,G=0.000000,B=0.042793,A=1.000000)" true))

(event Custom|Target%20Acquired
  (bind _asbp_character_enemy (Utilities|Casting|CastToBP_Character_Enemy (Variables|Default|GetclosestEnemy)))
  (bind _output_get (Variables|Default|SetactiveTarget _asbp_character_enemy))
  (Development|PrintString (Utilities|String|Append "ACTIVE TARGET = " (Utilities|GetDisplayName _output_get)) true true "(R=0.009243,G=1.000000,B=0.000000,A=1.000000)")
  (Variables|Default|SethasTarget true)
  (bind _returnvalue (Utilities|Time|SetTimerbyEvent (EventDispatchers|CreateEvent :!event Custom|Fire%20Turret) 0.2 true)) ; Time determines rate of fire
  (Variables|Default|SetfireTimer _returnvalue)
  (Rendering|Components|Light|SetLightColor (Variables|Default|GetPointLight) "(R=0.112504,G=1.000000,B=0.000000,A=1.000000)" true)
  (Audio|Components|Audio|Play (Variables|Default|GetLockOnSound) 0.0))

(event Custom|Fire%20Turret
  (bind _projectilearrow (Variables|Default|GetProjectileArrow))
  (bind _projectilearrow_2 (Variables|Default|GetProjectileArrow))
  (bind _projectilearrow_3 (Variables|Default|GetProjectileArrow))
  (bind _returnvalue (Transformation|GetWorldLocation _projectilearrow))
  (bind _returnvalue_2 (Transformation|GetWorldLocation _projectilearrow_3))
  ;[1 0.02053 0] Fire
  (bind _outhit (Collision|LineTraceForObjects _returnvalue (+ _returnvalue (* (Math|Vector|GetForwardVector _projectilearrow) 2.2e+04)) (Utilities|Array|MakeArray "ObjectTypeQuery3" "ObjectTypeQuery5") false 0 "None"))
  (if (!= (.HitActor (Collision|BreakHitResult _outhit)) (Variables|Default|GetowningCart))
    (Default|BulletProjectile (Variables|Default|GetBPC_Attacks) (Math|Transform|MakeTransform _returnvalue_2 (Math|Rotator|FindLookatRotation _returnvalue_2 (Transformation|GetActorLocation (Variables|Default|GetclosestEnemy))) "1.000000,1.000000,1.000000"))
    (Components|Activation|Activate (Variables|Default|GetNE_MuzzleFlash) true)
    (Niagara|SpawnSystematLocation "/Game/Characters/Player/Cart/Attachments/Turret/NS_GunSmoke.NS_GunSmoke" (Transformation|GetWorldLocation _projectilearrow_2) (Transformation|GetWorldRotation _projectilearrow_2))
    (Audio|Components|Audio|Play (Variables|Default|GetTurretShotSound) 0.0)))

(event Custom|Destroy%20Turret
  (Utilities|FlowControl|Sequence
    (:then_0
      (Utilities|Time|ClearandInvalidateTimerbyHandle (Variables|Default|GetfireTimer))
      (Utilities|Time|ClearandInvalidateTimerbyHandle (Variables|Default|GetaimingTimer))
      (Utilities|Time|ClearandInvalidateTimerbyHandle (Variables|Default|GetsenseNearbyTimer)))
    (:then_1
      (Components|DestroyComponent (Variables|Default|GetPointLight))
      (Audio|Components|Audio|Play (Variables|Default|GetSpeaker) 0.0)
      (Utilities|FlowControl|Delay 2.0)
      (Components|Activation|Deactivate (Variables|Default|GetNE_Fire)))
    (:then_2
      (Physics|SetSimulatePhysics (Variables|Default|GetturretBody) true)
      (Physics|SetPhysicsLinearVelocity (Variables|Default|GetturretHead) (Transformation|GetComponentVelocity (Variables|Default|GetWeapon)) false "None"))))

(event EventSetDelayTillDetach
  (params (time :type Float%20%28double-precision%29))
  (|CallParentFunction time)
  (if (!= 0.0 (Variables|Default|GettimeTillDetach))
    (Utilities|FlowControl|Delay (* (Variables|Default|GettimeTillDetach) 0.6))
    (Components|Activation|Activate (Variables|Default|GetNE_Fire) false)))

(event EventOnDetach
  (|CallParentFunction)
  (CallFunction|DestroyTurret))

(event EventBeginPlay
  (Utilities|FlowControl|Sequence
    (:then_0
      (bind _asbp_player_cart (Utilities|Casting|CastToBP_PlayerCart (Components|GetOwner))
        (:then
          (Variables|Default|SetowningCart _asbp_player_cart)
          (Variables|Default|SetownedByCart true))
        (:CastFailed
          (Development|PrintString "Cart is NOT turret OWNER!" true true "(R=1.000000,G=0.115187,B=0.000000,A=1.000000)")
          (Variables|Default|SetownedByCart false))))
    (:then_1
      (bind _returnvalue (Utilities|Time|SetTimerbyEvent (EventDispatchers|CreateEvent :!event Custom|Sense%20Nearby%20Targets) 0.25 true true))
      (Variables|Default|SetsenseNearbyTimer _returnvalue)
      (bind _returnvalue_2 (Utilities|Time|SetTimerbyEvent (EventDispatchers|CreateEvent :!event Custom|Aim%20At%20Target) 0.001 true true))
      (Variables|Default|SetaimingTimer _returnvalue_2))))

(fn ConstructionScript
  (|CallParentFunction))