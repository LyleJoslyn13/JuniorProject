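; Breakable armor piece for the player's cart that comes off when a projectile hits it.
; On the first hit by a BP_Projectile_Base, it sends a detach message to its owner, makes the armor block WorldStatic, then destroys itself after a short delay.
; Health, damage, team and attack-token functions are stubs returning zero or false, so the piece tracks no health of its own.
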(event Collision|EventHit
  (params (MyComp :type Primitive%20Component%20Object%20Reference) (Other :type Actor%20Object%20Reference) (OtherComp :type Primitive%20Component%20Object%20Reference) (bSelfMoved :type Boolean) (HitLocation :type Vector :default "0, 0, 0") (HitNormal :type Vector :default "0, 0, 0") (NormalImpulse :type Vector :default "0, 0, 0") (Hit :type Hit%20Result%20Structure%20%28by%20ref%29))
  (if (Class|GameplayStatics|ObjectIsA Other "/Game/Universal_Systems/Projectiles/BP_Projectile_Base.BP_Projectile_Base_C")
    (Utilities|FlowControl|DoOnce false
      (:Completed
        (Class|BPIInteractive|DetachArmor(Message) (Components|GetOwner) self)
        (Collision|SetCollisionResponsetoChannel (Variables|Default|GetArmor) "ECC_WorldStatic" "ECR_Block")
        (Utilities|FlowControl|Delay 5.0)
        (Actor|DestroyActor)))))

(fn ConstructionScript)

(fn GetCurrentHealth
  (return 0.0))

(fn GetMaxHealth
  (return 0.0))

(fn GetTeamNumber
  (return 0))

(fn Heal
  (params (AmountToHeal :type Float%20%28double-precision%29))
  (return 0.0))

(fn IsAttacking
  (return false))

(fn IsDead
  (return false))

(fn ReserveAttackToken
  (params (Amount :type Integer))
  (return false))

(fn TakeDamage
  (params (Damageinfo :type S%20Damage%20Info%20Structure) (DamageCausingActor :type Actor%20Object%20Reference) (DamageCausingComponent :type Object%20Object%20Reference))
  (return false))