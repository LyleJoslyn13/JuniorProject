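; Destructible post for enemy sentry platforms, built on a Geometry Collection that shatters when struck hard enough.
; A component hit above an impulse threshold fires once, applying a kinematic field and a radial impulse at the impact point.
; It also spawns an FS_MasterField field actor there, then signals the break through BreakingPost.
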(event OnComponentHit(GC_BP_DestructiblePost)
  (params (HitComponent :type Primitive%20Component%20Object%20Reference) (OtherActor :type Actor%20Object%20Reference) (OtherComp :type Primitive%20Component%20Object%20Reference) (NormalImpulse :type Vector :default "0, 0, 0") (Hit :type Hit%20Result%20Structure%20%28by%20ref%29))
  (bind _location (Collision|BreakHitResult Hit))
  (if (>= (Math|Vector|VectorLength NormalImpulse) 1e+04)
    (Utilities|FlowControl|DoOnce false
      (:Completed
        (Class|GeometryCollectionComponent|ApplyKinematicField (Variables|Default|GetGC_BP_DestructiblePost) 1e+03 _location)
        (Physics|AddRadialImpulse (Variables|Default|GetGC_BP_DestructiblePost) _location 1.0 1e+04 "RIF_Constant" false)
        (Game|SpawnActorfromClass "/Engine/EditorResources/FieldNodes/FS_MasterField.FS_MasterField_C" (Math|Conversions|ToTransform(Vector) _location) "Undefined" "MultiplyWithRoot" 0 0)
        (Default|CallBreakingPost)))))

(fn ConstructionScript)