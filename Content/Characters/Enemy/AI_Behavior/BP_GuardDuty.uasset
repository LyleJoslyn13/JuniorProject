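; BP_GuardDuty defines a spline-based patrol route for enemy guard AI, tracking the current waypoint.
; IncrementPatrolRoute steps the index along the GuardDuty spline, then either reverses at the last point or loops to the first, depending on LoopPathOnComplete.
; Looping sets Direction to a negative full-route step, so the next increment lands on index zero.
; GetSplinePointPositionAndRotation returns the current point's world location and the FacingDirection component's world location as a post facing target.
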(event Custom|IncrementPatrolRoute
  (bind _output_get (Variables|Default|SetPatrolIndex (+ (Variables|Default|GetPatrolIndex) (Variables|Default|GetDirection))))
  (if (== _output_get (- (Spline|GetNumberOfSplinePoints (Variables|Default|GetGuardDuty)) 1))
    (if (Variables|Default|GetloopPathOnComplete) ; If true, go back to the first index point \nafter reaching the last one. Otherwise, \ngo the previous index point from the last one \nand work way back to the first.
      (Variables|Default|SetDirection (* (- (Spline|GetNumberOfSplinePoints (Variables|Default|GetGuardDuty)) 1) -1))
      (else
        (Variables|Default|SetDirection -1)))
    (elif (== (Variables|Default|GetPatrolIndex) 0)
      (Variables|Default|SetDirection 1))))

(fn ConstructionScript)

(fn GetSplinePointPositionandRotation
  (return (Spline|GetLocationatSplinePoint (Variables|Default|GetGuardDuty) (Variables|Default|GetPatrolIndex) "World") (Transformation|GetWorldLocation (Variables|Default|GetFacingDirection))))