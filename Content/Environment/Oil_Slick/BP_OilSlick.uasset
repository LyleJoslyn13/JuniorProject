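; BP_OilSlick is an oil slick decal actor that explodes and burns when its Ignite event is called.
; Ignite spawns scaled explosion and fire emitters at the decal's location, fires the RadialForce impulse and plays both sounds there.
; The decal then fades out quickly and destroys the actor, while the effects are spawned at world locations independently of it.
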(event EventIgnite
  (bind _decal (Variables|Decal|GetDecal))
  (bind _returnvalue (Transformation|GetWorldLocation _decal))
  (Effects|SpawnEmitteratLocation "/Game/Environment/Oil_Slick/P_OilExplosion.P_OilExplosion" (Transformation|GetWorldLocation (Variables|Decal|GetDecal)) "0, 0, 0" "8.000000,8.000000,8.000000")
  (Effects|SpawnEmitteratLocation "/Game/Environment/Oil_Slick/P_OilFire.P_OilFire" (Transformation|GetWorldLocation (Variables|Decal|GetDecal)) "0, 0, 0" "8.000000,3.000000,8.000000")
  (Rendering|Components|Decal|SetFadeOut (Variables|Decal|GetDecal) 0.0 0.5 true)
  (Class|RadialForceComponent|FireImpulse (Variables|Default|GetRadialForce))
  (Audio|PlaySoundatLocation "/Game/Sounds/Explosion/OilExplosion/OilExplosion_Cue.OilExplosion_Cue" _returnvalue "0, 0, 0" 1.0 1.0 0.0 0 0 0 0)
  (Audio|PlaySoundatLocation "/Game/Sounds/Fire/QuickFire_Cue.QuickFire_Cue" _returnvalue "0, 0, 0" 1.0 1.0 0.0 0 0 0 0))

(fn ConstructionScript)