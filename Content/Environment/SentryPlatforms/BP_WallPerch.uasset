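; BP_WallPerch is a sentry platform with a destructible post child actor that can collapse and drop characters standing on it.
; On BeginPlay it binds to the post's breaking event.
; Collapse turns on physics for the platform, changes its tag to "None" and starts a delayed fade-away.
; It then box-traces physics bodies above its root and ragdolls any BP_Character_Base found.
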(event Custom|Collapse
  (bind _defaultsceneroot (Variables|Default|GetDefaultSceneRoot))
  (bind _returnvalue (Transformation|GetWorldLocation _defaultsceneroot))
  (bind _returnvalue_2 (+ _returnvalue "0.000000,0.000000,100.000000"))
  (Utilities|FlowControl|Sequence
    (:then_0
      (Physics|SetSimulatePhysics (Variables|Default|GetPlatform) true)
      (Variables|/Script/Engine.ActorComponent|SetComponentTags (Variables|Default|GetPlatform) (Utilities|Array|MakeArray "None"))
      (Default|FadeAwayComponent (Variables|Default|GetBP_FadeAway) (Variables|Default|GetPlatform) 5.0))
    (:then_1
      (bind _outhits (Class|KismetSystemLibrary|BoxTraceMultiforObjects _returnvalue_2 _returnvalue_2 "150.000000,250.000000,100.000000" (Transformation|GetWorldRotation _defaultsceneroot) (Utilities|Array|MakeArray (Utilities|Enum|LiteralenumEObjectTypeQuery "ObjectTypeQuery4")) false 0 "None" true))
      (for _array_element _outhits
        (if (Class|GameplayStatics|ObjectIsA (.HitActor (Collision|BreakHitResult _array_element)) "/Game/Characters/CharacterBase/BP_Character_Base.BP_Character_Base_C")
          (bind _asbp_character_base (Utilities|Casting|CastToBP_Character_Base (.HitActor (Collision|BreakHitResult _array_element))))
          (Default|StartRagdoll _asbp_character_base))))))

(event EventBeginPlay
  (bind _asbp_destructible_post (Utilities|Casting|CastToBP_DestructiblePost (Variables|/Script/Engine.ChildActorComponent|GetChildActor (Variables|Default|GetBP_DestructiblePost))))
  (EventDispatchers|BindEventtoBreakingPost _asbp_destructible_post (EventDispatchers|CreateEvent :!event Custom|Collapse)))

(fn ConstructionScript)