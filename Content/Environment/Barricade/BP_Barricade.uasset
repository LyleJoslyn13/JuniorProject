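; BP_Barricade is a destructible stone barricade built on a Geometry Collection that breaks apart and fades away.
; Each Chaos break event plays a cracking sound, spawns rock puff particles at the break and increments a count of broken pieces.
; Once the count reaches a threshold, it fires React once, which crumbles the active clusters and starts a delayed fade-away through BPFadeAway.
; The break counter serves as a workaround for tracking how fractured the object is.
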(event OnChaosBreakEvent(GC_Barricade_Low)
  (params (BreakEvent :type Chaos%20Break%20Event%20Structure%20%28by%20ref%29))
  (bind (_component _location) (Utilities|Struct|BreakChaosBreakEvent BreakEvent))
  (Audio|PlaySoundatLocation "/Game/Sounds/Rock/StoneCracking_Cue.StoneCracking_Cue" _location "0, 0, 0" 1.0 1.0 0.0 0 0 0 0)
  (Effects|SpawnEmitterAttached "/Game/Environment/Barricade/Assets/KyleBarrier/P_RockPuff.P_RockPuff" _component "None" _location "0, 0, 0" "1.000000,1.000000,1.000000" "KeepWorldPosition")
  (bind _result (Math|Float|IncrementFloat (Variables|Default|GetnumberOfPiecesBroken)) ; (I hate this, but I can't\nfind another way to track\nhow much the object has fractured)
    (:%20%20
      (if (>= _result 7.0)
        (Utilities|FlowControl|DoOnce false
          (:Completed
            (CallFunction|React)))))))

(event EventReact
  (Utilities|FlowControl|DoOnce false
    (:Completed
      (Class|GeometryCollectionComponent|CrumbleActiveClusters (Variables|Default|GetGC_Barricade_Low))
      (Default|FadeAwayActor (Variables|Default|GetBP_FadeAway) (Variables|Default|GetGC_Barricade_Low) 5.0))))

(fn ConstructionScript)