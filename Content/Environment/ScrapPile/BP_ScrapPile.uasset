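; BP_ScrapPile is a scrap pile prop that randomizes its meshes and turns them into physics debris on BeginPlay.
; It loops over pile, middle and falling sections, with middle gated by a flag and falling by a flag plus a coin flip.
; Each processed section's child mesh components get random scrap meshes and are collected in ScrapItems.
; Physics starts only after all sections finish, because simulating detaches components and would skip children.
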(event Custom|Simulate%20Scrap
  ;[1 1 1] This has to be done seperatley, otherwise if objects are simulated after they are set, then they will be removed from the children components. Which causes certain children to get skipped.
  (bind _result (Utilities|Set|ToArray (Variables|Default|GetscrapItems)))
  (for _array_element _result
    (Physics|SetSimulatePhysics _array_element true)))

(event Custom|Set%20Random%20Scrap%20Mesh
  (params (staticMesh :type Scene%20Component%20Object%20Reference) (scrapSection :type E_ScrapSection%20Enum :default "NewEnumerator0"))
  (bind _returnvalue (Math|Random|RandomIntegerinRange 0 2))
  (bind _returnvalue_2 (Utilities|Select :Index _returnvalue :Option%200 "/Game/Environment/ScrapPile/Scrap_Mesh_SheetMetal.Scrap_Mesh_SheetMetal" :Option%201 "/Game/Environment/ScrapPile/Scrap_Mesh_WoodPallet1.Scrap_Mesh_WoodPallet1" :Option%202 "/Game/Environment/ScrapPile/Scrap_Mesh_WoodPallet2.Scrap_Mesh_WoodPallet2"))
  (bind _asstatic_mesh_component (Utilities|Casting|CastToStaticMeshComponent staticMesh))
  (Utilities|Set|Add (Variables|Default|GetscrapItems) _asstatic_mesh_component)
  (Components|StaticMesh|SetStaticMesh _asstatic_mesh_component (Utilities|Select :Index scrapSection :NewEnumerator0 _returnvalue_2 :NewEnumerator1 (Utilities|Select :Index (Math|Random|RandomIntegerinRange 0 1) :Option%200 "/Game/Environment/ScrapPile/mesh_Barrel.mesh_Barrel" :Option%201 "/Game/Environment/ScrapPile/Scrap_Mesh_Spring.Scrap_Mesh_Spring" :Option%202 "/Game/Environment/ScrapPile/Scrap_Mesh_WoodPallet2.Scrap_Mesh_WoodPallet2") :NewEnumerator2 _returnvalue_2)))

(event Custom|Randomize%20Scrap%20Pile
  (params (scrapSection :type E_ScrapSection%20Enum :default "NewEnumerator0"))
  (for _array_element (Components|GetChildrenComponents (Utilities|Select :Index scrapSection :NewEnumerator0 (Variables|Default|GetScrapPile) :NewEnumerator1 (Variables|Default|GetScrapMiddle) :NewEnumerator2 (Variables|Default|GetScrapFalling)) false)
    (CallFunction|SetRandomScrapMesh _array_element scrapSection)))

(event EventBeginPlay
  (bind _enumvalue (|ForEachE_ScrapSection)
    (:LoopBody
      (switch Utilities|FlowControl|Switch|SwitchonE_ScrapSection _enumvalue
        (:NewEnumerator0
          (CallFunction|RandomizeScrapPile _enumvalue :!label _label))
        (:NewEnumerator1
          (if (Variables|Default|GetsetMiddleScrap)
            (goto _label)))
        (:NewEnumerator2
          (if (and (Variables|Default|GetsetFallingScrap) (Math|Random|RandomBool))
            (goto _label)))))
    (:then
      (CallFunction|SimulateScrap)
      (bind _result (Utilities|Set|ToArray (Variables|Default|GetscrapItems)))
      (Variables|Default|SetnearbyScrapChildren _result))))

(fn ConstructionScript)