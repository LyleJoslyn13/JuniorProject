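; Attack component that spawns bullet, homing ninja star and trashball projectiles that ignore collision with the owner.
; Bound impact handlers report damage events for AI sensing, but only the ninja star's handler also sends a TakeDamage message.
; Bullet shots and impacts make noise attributed to player 0.
; OnAttackEnded fires on impact for bullets and stars, but right after spawn for trashballs.
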(event Custom|Bullet%20Projectile
  (params (SpawnTransform :type Transform) (Target :type Actor%20Object%20Reference) (DamageInfo :type S%20Damage%20Info%20Structure))
  (bind _returnvalue (Game|SpawnActorfromClass "/Game/Universal_Systems/Projectiles/BP_Projectile_Bullet.BP_Projectile_Bullet_C" SpawnTransform "Undefined" "MultiplyWithRoot" (Components|GetOwner) 1e+04 0.0 Target false true 0))
  (EventDispatchers|BindEventtoOnProjectileImpact _returnvalue (delegate Custom|On%20Bullet%20Impact))
  (Collision|IgnoreActorwhenMoving (Variables|/Game/Universal_Systems/Projectiles/BP_Projectile_Base.BP_Projectile_Base_C|GetBoxCollision _returnvalue) (Components|GetOwner) true)
  (Class|Actor|MakeNoise _returnvalue 1.0 (Game|GetPlayerCharacter 0) (.Location (Math|Transform|BreakTransform SpawnTransform)) 0.0 "None") ; Noise from gunshot
)

(event Custom|On%20Ninja%20Star%20Impact
  (params (OtherActor :type Actor%20Object%20Reference) (Hit :type Hit%20Result%20Structure))
  (bind _hitactor (Collision|BreakHitResult Hit))
  (bind _returnvalue (Components|GetOwner))
  (Class|BPIDamagable|TakeDamage(Message) _hitactor (stale Custom|Ninja%20Star DamageInfo) _returnvalue (stale Custom|Ninja%20Star _returnvalue))
  (Class|AISenseDamage|ReportDamageEvent _hitactor _returnvalue (.AmountOfDamage (Utilities|Struct|BreakS_DamageInfo (stale Custom|Ninja%20Star DamageInfo))) (Transformation|GetActorLocation (Components|GetOwner)) "0, 0, 0" "None")
  (Default|CallOnAttackEnded))

(event Custom|On%20Bullet%20Impact
  (params (OtherActor :type Actor%20Object%20Reference) (Hit :type Hit%20Result%20Structure))
  (bind (_bblockinghit _binitialoverlap _time _distance _location _impactpoint _normal _impactnormal _physmat _hitactor) (Collision|BreakHitResult Hit))
  (Class|AISenseDamage|ReportDamageEvent _hitactor (Components|GetOwner) (.AmountOfDamage (Utilities|Struct|BreakS_DamageInfo (stale Custom|Bullet%20Projectile DamageInfo))) (Transformation|GetActorLocation (Components|GetOwner)) "0, 0, 0" "None")
  (Class|Actor|MakeNoise _hitactor 0.25 (Game|GetPlayerCharacter 0) _location 0.0 "None") ; Noise from bullet impact
  (Default|CallOnAttackEnded))

(event Custom|Ninja%20Star
  (params (SpawnTransform :type Transform) (Target :type Actor%20Object%20Reference) (DamageInfo :type S%20Damage%20Info%20Structure))
  (bind _returnvalue (Game|SpawnActorfromClass "/Game/Universal_Systems/Projectiles/BP_Projectile_NinjaStar.BP_Projectile_NinjaStar_C" SpawnTransform "Undefined" "MultiplyWithRoot" (Components|GetOwner) 1.5e+03 1.0 Target true false 0))
  (EventDispatchers|BindEventtoOnProjectileImpact _returnvalue (delegate Custom|On%20Ninja%20Star%20Impact))
  (Collision|IgnoreActorwhenMoving (Variables|/Game/Universal_Systems/Projectiles/BP_Projectile_Base.BP_Projectile_Base_C|GetBoxCollision _returnvalue) (Components|GetOwner) true))

(event Custom|On%20Trashball%20Impact
  (params (OtherActor :type Actor%20Object%20Reference) (Hit :type Hit%20Result%20Structure))
  (Class|AISenseDamage|ReportDamageEvent (.HitActor (Collision|BreakHitResult Hit)) (Components|GetOwner) (.AmountOfDamage (Utilities|Struct|BreakS_DamageInfo (stale Custom|Trashball damageInfo))) (Transformation|GetActorLocation (Components|GetOwner)) "0, 0, 0" "None"))

(event Custom|Trashball
  (params (spawnTransform :type Transform) (owner :type Actor%20Object%20Reference) (trailColor :type Linear%20Color%20Structure :default "(R=1.000000,G=1.000000,B=1.000000,A=1.000000)") (speed :type Float%20%28double-precision%29) (gravity :type Float%20%28double-precision%29) (target :type Actor%20Object%20Reference) (damageInfo :type S%20Damage%20Info%20Structure))
  (bind _returnvalue (Game|SpawnActorfromClass "/Game/Universal_Systems/Projectiles/BP_Projectile_Trashball.BP_Projectile_Trashball_C" spawnTransform "Undefined" "MultiplyWithRoot" owner trailColor speed gravity target false false 0))
  (EventDispatchers|BindEventtoOnProjectileImpact _returnvalue (delegate Custom|On%20Trashball%20Impact))
  (Collision|IgnoreActorwhenMoving (Variables|/Game/Universal_Systems/Projectiles/BP_Projectile_Base.BP_Projectile_Base_C|GetBoxCollision _returnvalue) owner true)
  (Collision|IgnoreActorwhenMoving (Variables|/Game/Universal_Systems/Projectiles/BP_Projectile_Base.BP_Projectile_Base_C|GetBoxCollision _returnvalue) (Components|GetOwner) true)
  (Variables|Default|SetprojectileRef _returnvalue)
  (Default|CallOnAttackEnded))