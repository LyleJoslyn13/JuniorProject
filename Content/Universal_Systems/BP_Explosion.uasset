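; BP_Explosion is a one-shot explosion actor that applies damage, physics impulse and effects on BeginPlay, then destroys itself.
; A sphere trace finds physics, vehicle and destructible objects, sending each unique actor a TriggerDestructions message and damaging BP_Character_Base characters.
; It then spawns a radius-scaled emitter, plays sound and fires a radial force configured from its radius and strength.
; After a short delay it spawns a BP_Decal scorch mark, optionally inheriting rotation.
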(event EventBeginPlay
  (bind _explosionroot (Variables|Default|GetexplosionRoot))
  (bind _radialforceexplosion (Variables|Default|GetradialForceExplosion))
  (bind _explosionroot_2 (Variables|Default|GetexplosionRoot))
  (bind _explosionroot_3 (Variables|Default|GetexplosionRoot))
  (bind _returnvalue (Transformation|GetWorldTransform _explosionroot_2))
  (bind _returnvalue_2 (Transformation|GetWorldLocation _explosionroot_3))
  (bind _returnvalue_3 (Transformation|GetWorldLocation _explosionroot))
  (bind (_location _rotation _scale) (Math|Transform|BreakTransform _returnvalue))
  (Variables|/Script/Engine.RadialForceComponent|SetRadius _radialforceexplosion (Variables|Default|GetexplosionRadius))
  (Variables|/Script/Engine.RadialForceComponent|SetImpulseStrength _radialforceexplosion (Variables|Default|GetexplosionStrength))
  (Utilities|FlowControl|Sequence
    (:then_0
      (bind _outhits (Collision|MultiSphereTraceForObjects _returnvalue_2 _returnvalue_2 (Variables|Default|GetexplosionRadius) (Utilities|Array|MakeArray "ObjectTypeQuery4" "ObjectTypeQuery5" "ObjectTypeQuery6") false 0 "None" :!pinned true)) ; Explosion Radius
      (for _array_element _outhits
        (if (== (Utilities|Array|FindItem (Variables|Default|GethitActorsArray) (.HitActor (Collision|BreakHitResult _array_element))) -1) ; Only hits each actor once
          (Utilities|Array|AddUnique (Variables|Default|GethitActorsArray) (.HitActor (Collision|BreakHitResult _array_element)))
          (Class|BPIDestructible|React(Message) (.HitActor (Collision|BreakHitResult _array_element)) (Variables|Default|GettriggerDestructions?) :!pinned true) ; React if Destructible
          (if (and (!= (Variables|Default|GetexplosionDamage) 0.0) (Class|GameplayStatics|ObjectIsA (.HitActor (Collision|BreakHitResult _array_element)) "/Game/Characters/CharacterBase/BP_Character_Base.BP_Character_Base_C"))
            (bind _asbp_character_base (Utilities|Casting|CastToBP_Character_Base (.HitActor (Collision|BreakHitResult _array_element))))
            (Default|TakeDamage _asbp_character_base (Utilities|Struct|MakeS_DamageInfo (Variables|Default|GetexplosionDamage) "NewEnumerator2" "NewEnumerator0" true false false true) self (Variables|Default|GetexplosionRoot) :!pinned true) ; Damage Characters
          )))
      (Utilities|Array|Clear (Variables|Default|GethitActorsArray)))
    (:then_1
      (Effects|SpawnEmitteratLocation (Variables|Default|GetexplosionEmitter) _returnvalue_3 "0, 0, 0" (Math|Conversions|ToVector(Float) (* (Variables|Default|GetexplosionRadius) 0.01)) :!pinned true) ; Explosion Emitter
      (Audio|PlaySoundatLocation (Variables|Default|GetexplosionSound) _returnvalue_3 "0, 0, 0" 1.0 1.0 0.0 0 0 0 0 :!pinned true) ; Explosion Sound
      (Class|RadialForceComponent|FireImpulse (Variables|Default|GetRadialForceExplosion))
      (Utilities|FlowControl|Delay 0.1)
      (Game|SpawnActorfromClass "/Game/Universal_Systems/Explosion/BP_Decal.BP_Decal_C" (select (Variables|Default|GetdecalInheritRotation?) _returnvalue (Math|Transform|MakeTransform _location "0, 0, 0" _scale)) "Undefined" "MultiplyWithRoot" 0 (Variables|Default|GetscortchDecal) 0 :!pinned true) ; Decal
      (Actor|DestroyActor))))

(fn ConstructionScript)