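; Trashball projectile that flies with a colored smoke trail and becomes a physics object on impact.
; The first hit enables gravity physics, then tags the collision "NoHit" and stops the trail, after a short delay for velocity damage unless it struck cart armor.
; On spawn, a short forward trace catches obstacles too close for normal collision, switching to physics early and converting speed into an impulse.
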(event OnComponentHit(BoxCollision)
  (params (HitComponent :type Primitive%20Component%20Object%20Reference) (OtherActor :type Actor%20Object%20Reference) (OtherComp :type Primitive%20Component%20Object%20Reference) (NormalImpulse :type Vector :default "0, 0, 0") (Hit :type Hit%20Result%20Structure%20%28by%20ref%29))
  (Utilities|FlowControl|DoOnce false
    (:Completed
      (CallFunction|EnablePhysics&Gravity)
      (if (not (Class|GameplayStatics|ObjectIsA OtherActor "/Game/Characters/Player/Cart/Attachments/Armor/BP_CartArmor.BP_CartArmor_C")) ; deactivates projectile immeditally\nif hitting a 'Cart Armor'
        (Utilities|FlowControl|Delay 0.2) ; needed for velocity damage
      )
      (Variables|/Script/Engine.ActorComponent|SetComponentTags (Variables|Default|GetBoxCollision) (Utilities|Array|MakeArray "NoHit"))
      (Components|Activation|Deactivate (Variables|Default|GetNS_TrailSmoke)))))

(event EventBeginPlay
  (Effects|Components|ParticleSystem|SetColorParameter (Variables|Default|GetNS_TrailSmoke) "Color" (Variables|Default|GetTrailColor))
  (|CallParentFunction)
  (CallFunction|CheckDistanceforPhysicsSpawn))

(fn ConstructionScript
  (|CallParentFunction))

(fn CheckDistanceforPhysicsSpawn
  (bind _boxcollision (Variables|Default|GetBoxCollision))
  (bind _returnvalue (Math|Vector|GetForwardVector _boxcollision))
  (bind _returnvalue_2 (Transformation|GetWorldLocation _boxcollision))
  ;[1 1 1] If current path will lead to a collision sooner than what the Unreal can caluclate, then pre-emptivley enable physics and convert speed to impulse.
  (bind _returnvalue_3 (Collision|LineTraceByChannel _returnvalue_2 (+ _returnvalue_2 (* _returnvalue 5e+02)) "TraceTypeQuery1" false 0 "None"))
  (if _returnvalue_3
    (CallFunction|EnablePhysics&Gravity)
    (Physics|AddImpulse (Variables|Default|GetBoxCollision) (* (Variables|Default|GetSpeed) _returnvalue) "None" true)))