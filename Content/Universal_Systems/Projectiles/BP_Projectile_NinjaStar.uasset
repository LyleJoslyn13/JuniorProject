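; Ninja star projectile Blueprint that handles the star's in-flight orientation and spin.
; Each Tick, it turns the actor toward its velocity using only the roll and yaw of a look-at rotation, leaving pitch out.
; It then spins the mesh by a fixed local roll step per frame, so spin speed depends on frame rate.
; It defines no hit or damage logic itself.
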(event EventBeginPlay)

(event Collision|EventActorBeginOverlap
  (params (OtherActor :type Actor%20Object%20Reference)))

(event EventTick
  (params (DeltaSeconds :type Float%20%28single-precision%29))
  (bind _returnvalue (Transformation|GetActorLocation))
  (bind _returnvalue_2 (Transformation|GetVelocity))
  (bind _returnvalue_3 (+ _returnvalue _returnvalue_2))
  (bind _returnvalue_4 (Math|Rotator|FindLookatRotation _returnvalue _returnvalue_3))
  (bind (_roll _pitch _yaw) (Math|Rotator|BreakRotator _returnvalue_4))
  (Transformation|SetActorRotation (Math|Rotator|MakeRotator _roll 0.0 _yaw))
  (Transformation|AddLocalRotation (Variables|Character|GetMesh) (Math|Rotator|MakeRotator -2e+01 0.0 0.0) false false))

(fn ConstructionScript
  (|CallParentFunction))