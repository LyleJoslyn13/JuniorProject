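; Attack component that fires bullet and homing ninja star projectiles on behalf of its owning actor.
; Each attack spawns a targeted projectile, makes the owner's capsule ignore it and binds an impact handler that reports damage and signals OnAttackEnded.
; Only the ninja star impact also sends a TakeDamage message to the hit actor.
; Bullets emit noise when fired and on impact, instigated by the player character.
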(event Custom|BulletProjectile
  (params (SpawnTransform :type Transform) (Target :type Actor%20Object%20Reference) (Damageinfo :type S%20Damage%20Info%20Structure))
  (bind _returnvalue (Game|SpawnActorfromClass "/Game/Universal_Systems/Projectiles/BP_Projectile_Bullet.BP_Projectile_Bullet_C" SpawnTransform "Undefined" "MultiplyWithRoot" (Components|GetOwner) 4e+03 0.0 Target false true 0))
  (EventDispatchers|BindEventtoOnProjectileImpact _returnvalue (delegate Custom|OnBulletImpact))
  (Collision|IgnoreActorwhenMoving (Actor|GetComponentbyClass (Components|GetOwner) "/Script/Engine.CapsuleComponent") _returnvalue true)
  (Class|Actor|MakeNoise _returnvalue 1.0 (Game|GetPlayerCharacter 0) (.Location (Math|Transform|BreakTransform SpawnTransform)) 0.0 "None") ; Noise from gunshot
)

(event Custom|OnBulletImpact
  (params (OtherActor :type Actor%20Object%20Reference) (Hit :type Hit%20Result%20Structure))
  (bind (_bblockinghit _binitialoverlap _time _distance _location _impactpoint _normal _impactnormal _physmat _hitactor) (Collision|BreakHitResult Hit))
  (Class|AISenseDamage|ReportDamageEvent _hitactor (Components|GetOwner) (.AmountOfDamage (Utilities|Struct|BreakS_DamageInfo (stale Custom|BulletProjectile Damageinfo))) (Transformation|GetActorLocation (Components|GetOwner)) "0, 0, 0" "None")
  (Class|Actor|MakeNoise _hitactor 0.25 (Game|GetPlayerCharacter 0) _location 0.0 "None") ; Noise from bullet impact
  (Default|CallOnAttackEnded))

(event Custom|NinjaStar
  (params (SpawnTransform :type Transform) (Target :type Actor%20Object%20Reference) (Damageinfo :type S%20Damage%20Info%20Structure))
  (bind _returnvalue (Game|SpawnActorfromClass "/Game/Universal_Systems/Projectiles/BP_Projectile_NinjaStar.BP_Projectile_NinjaStar_C" SpawnTransform "Undefined" "MultiplyWithRoot" (Components|GetOwner) 1.5e+03 0.01 Target true false 0))
  (EventDispatchers|BindEventtoOnProjectileImpact _returnvalue (delegate Custom|OnNinjaStarImpact))
  (Collision|IgnoreActorwhenMoving (Actor|GetComponentbyClass (Components|GetOwner) "/Script/Engine.CapsuleComponent") _returnvalue true))

(event Custom|OnNinjaStarImpact
  (params (OtherActor :type Actor%20Object%20Reference) (Hit :type Hit%20Result%20Structure))
  (bind _returnvalue (Components|GetOwner))
  (bind _hitactor (Collision|BreakHitResult Hit))
  (Class|BPIDamagable|TakeDamage(Message) _hitactor (stale Custom|NinjaStar Damageinfo) _returnvalue (stale Custom|NinjaStar _returnvalue))
  (Class|AISenseDamage|ReportDamageEvent _hitactor _returnvalue (.AmountOfDamage (Utilities|Struct|BreakS_DamageInfo (stale Custom|NinjaStar Damageinfo))) (Transformation|GetActorLocation (Components|GetOwner)) "0, 0, 0" "None")
  (Default|CallOnAttackEnded))