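; Base projectile actor that flies at a set speed and gravity, optionally homing on a Target.
; The construction script configures ProjectileMovement from its variables, including homing on the target's root component.
; On BeginPlay it ignores its owner, aims velocity once at any valid Target, and self-destructs after a timeout.
; On box hit it calls OnProjectileImpact, plays impact effect and sound, then destroys itself next tick.
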(event OnComponentHit(BoxCollision)
  (params (HitComponent :type Primitive%20Component%20Object%20Reference) (OtherActor :type Actor%20Object%20Reference) (OtherComp :type Primitive%20Component%20Object%20Reference) (NormalImpulse :type Vector :default "0, 0, 0") (Hit :type Hit%20Result%20Structure%20%28by%20ref%29))
  (bind _location (Collision|BreakHitResult Hit))
  (Default|CallOnProjectileImpact OtherActor Hit)
  (Effects|SpawnEmitteratLocation (Variables|Effects|GetImpactEffect) _location)
  (Audio|PlaySoundatLocation (Variables|Sounds|GetImpactSound) _location "0, 0, 0" 1.0 1.0 0.0 0 0 0 0)
  (Utilities|FlowControl|DelayUntilNextTick)
  (Actor|DestroyActor))

(event Custom|RotateToTarget
  ;[0 0 0] Gets target location and adjusts rotation to it's position (does not follow actor)
  (Variables|/Script/Engine.MovementComponent|SetVelocity (Variables|Default|GetProjectileMovement) (* (Math|Vector|GetUnitDirection(Vector) (Transformation|GetActorLocation) (Transformation|GetActorLocation (Variables|Target|GetTarget))) (Variables|ProjectileSettings|GetSpeed))))

(event EventBeginPlay
  (Utilities|FlowControl|Sequence
    (:then_0
      (Collision|IgnoreActorwhenMoving (Variables|Default|GetBoxCollision) (Components|GetOwner) true)
      (Variables|Target|GetTarget
        (:then
          (CallFunction|RotatetoTarget))
        (:else)))
    (:then_1
      (Utilities|FlowControl|Delay 15.0)
      (Actor|DestroyActor))))

(fn ConstructionScript
  (bind _projectilemovement (Variables|Default|GetProjectileMovement))
  (bind _speed (Variables|ProjectileSettings|GetSpeed))
  (Variables|/Script/Engine.ProjectileMovementComponent|SetInitialSpeed _projectilemovement _speed)
  (Variables|/Script/Engine.ProjectileMovementComponent|SetMaxSpeed _projectilemovement _speed)
  (Variables|/Script/Engine.ProjectileMovementComponent|SetProjectileGravityScale _projectilemovement (Variables|ProjectileSettings|GetGravity))
  (Variables|/Script/Engine.ProjectileMovementComponent|SetbRotationFollowsVelocity _projectilemovement (Variables|ProjectileSettings|GetrotationFollowsVelocity))
  ;[0 0 0] If there is a valid target and homing is 'True', set ProjectileMovement to homing and use the valid target as selected target
  (Variables|Target|GetTarget
    (:then
      (Variables|/Script/Engine.ProjectileMovementComponent|SetbIsHomingProjectile _projectilemovement (Variables|ProjectileSettings|GetisHoming))
      (Variables|/Script/Engine.ProjectileMovementComponent|SetHomingTargetComponent _projectilemovement (Variables|/Script/Engine.Actor|GetRootComponent (Variables|Target|GetTarget))))
    (:else)))