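; BP_FadeAway is a component that gradually fades a given mesh, then destroys its owning actor.
; FadeAwayActor makes dynamic instances of the mesh's materials, swapping any without a non-zero "Fade Amount" parameter for a warning material.
; After the given delay, a looping timer steps that parameter upward, disabling shadow casting at zero and destroying the owner at one.
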(event Custom|Fade%20Timer
  (Variables|Default|SettransitionValue (+ (Variables|Default|GettransitionValue) 0.1))
  (for _array_element (Variables|Default|GetdynamicMaterial_0)
    (Rendering|Material|SetScalarParameterValue _array_element "Fade Amount" (Variables|Default|GettransitionValue) :!class /Script/Engine.MaterialInstanceDynamic)
    (if (>= (Variables|Default|GettransitionValue) 0.0)
      (Utilities|FlowControl|Sequence
        (:then_0
          (Utilities|FlowControl|DoOnce false
            (:Completed
              (Rendering|SetCastShadow (Variables|Default|Getmesh) false))))
        (:then_1
          (if (>= (Variables|Default|GettransitionValue) 1.0)
            (Utilities|FlowControl|DelayUntilNextTick)
            (Actor|DestroyActor (Components|GetOwner))))))))

(event Custom|Fade%20Away%20Actor
  (params (meshToFade :type Mesh%20Component%20Object%20Reference) (delayBeforeFadeStarts :type Float%20%28double-precision%29))
  (Variables|Default|Setmesh meshToFade)
  (Variables|Default|SetdelayBeforeFadeStarts delayBeforeFadeStarts)
  (CallFunction|DetermineAmountOfMaterials))

(event Custom|Determine%20Amount%20of%20Materials
  (for (_array_element _array_index) (Rendering|Material|GetMaterials (Variables|Default|Getmesh))
    (bind _returnvalue (Rendering|Material|CreateDynamicMaterialInstance (Variables|Default|Getmesh) _array_index _array_element "None" :!class /Script/Engine.PrimitiveComponent))
    (bind _returnvalue_2 (Utilities|Array|AddUnique (Variables|Default|GetdynamicMaterial_0) _returnvalue))
    (bind _returnvalue_3 (Rendering|Material|GetScalarParameterValue _returnvalue "Fade Amount" :!class /Script/Engine.MaterialInstanceDynamic)) ; That parameter will ALWAYS start at -1\nif it exists within the parent. If this value \nis equal to 0, that means it does not contain\nthe proper parameter.
    (if (not (!= _returnvalue_3 0.0)) ; Contains parameter?
      (Utilities|Array|RemoveItem (Variables|Default|GetdynamicMaterial_0) _returnvalue)
      (bind _returnvalue_4 (Rendering|Material|CreateDynamicMaterialInstance (Variables|Default|Getmesh) _returnvalue_2 "/Game/Universal_Systems/FadeAway/M_MissingFadeWarning.M_MissingFadeWarning" "None" :!class /Script/Engine.PrimitiveComponent)) ; Change material to warning material
      (Utilities|Array|AddUnique (Variables|Default|GetdynamicMaterial_0) _returnvalue_4)))
  (Utilities|Time|SetTimerbyEvent (EventDispatchers|CreateEvent :!event Custom|Fade%20Timer) 0.1 true false (Variables|Default|GetdelayBeforeFadeStarts)))