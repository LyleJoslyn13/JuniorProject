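; Ability component for characters, providing bullet time, a Broken Instrument effect and invisibility, plus area stun and confuse of enemies.
; Bullet time uses a looping timer to ramp clamped global time dilation and pitch, notifying listeners through UpdateTimeMultiplier.
; Broken Instrument and Invisible run looping timers ended by retriggerable delays, the former with attached Niagara and sound.
; Stun and confuse share a sphere trace that deduplicates hits before triggering each enemy's reaction.
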(event Custom|Bullet%20Time
  (params (turnOffBulletTime :type Boolean))
  ;[1 0.1912 0] Bullet Time
  (if (not turnOffBulletTime)
    (Variables|Default|SetbulletTimeDirection -1.0)
    (else
      (Variables|Default|SetbulletTimeDirection 1.0)))
  (bind _returnvalue (Utilities|Time|SetTimerbyEvent (delegate Custom|Scale%20Time%20Speed) 0.01 true))
  (Variables|Default|SetbulletTimeTimer _returnvalue))

(event Custom|Scale%20Time%20Speed
  (bind _returnvalue (Class|GameplayStatics|GetGlobalTimeDilation))
  (bind _bullettimedirection (Variables|Default|GetbulletTimeDirection))
  (bind _returnvalue_2 (* _bullettimedirection 0.01))
  (bind _returnvalue_3 (+ _returnvalue _returnvalue_2))
  (bind _returnvalue_4 (Math|Float|Clamp(Float) _returnvalue_3 0.25))
  ;[1 0.1912 0] Bullet Time
  (Utilities|Time|SetGlobalTimeDilation _returnvalue_4)
  (Class|GameplayStatics|SetGlobalPitchModulation (Math|Float|MapRangeClamped (Class|GameplayStatics|GetGlobalTimeDilation) 1.0 0.25 1.0 0.75) 0.25)
  (Default|CallUpdateTimeMultiplier _returnvalue_4) ; Updates bound events to time change
  (if (or (and (<= _returnvalue_4 0.25) (< (Variables|Default|GetbulletTimeDirection) 0.0)) (and (>= _returnvalue_4 1.0) (> (Variables|Default|GetbulletTimeDirection) 0.0)))
    (Utilities|Time|ClearandInvalidateTimerbyHandle (Variables|Default|GetbulletTimeTimer))))

(event Custom|Broken%20Instrument
  (bind _returnvalue (Components|GetOwner))
  (bind _returnvalue_2 (Transformation|GetActorLocation _returnvalue))
  (bind (_asbp_character_base _bsuccess) (Utilities|Casting|CastToBP_Character_Base _returnvalue))
  (bind _rootcomponent (Variables|/Script/Engine.Actor|GetRootComponent _returnvalue))
  (bind _worldrotationsphere_forbrokeninstrument_ (Variables|/Game/Characters/CharacterBase/BP_Character_Base.BP_Character_Base_C|GetWorldRotationSphere%28ForBrokenInstrument%29 _asbp_character_base))
  (bind _returnvalue_3 (select _bsuccess _worldrotationsphere_forbrokeninstrument_ _rootcomponent))
  ;[0.08305 1 0] Broken Instrument
  (bind _returnvalue_4 (Niagara|SpawnSystemAttached "/Game/Universal_Systems/Abilities/NS_BrokenInstrument.NS_BrokenInstrument" _returnvalue_3 "None" _returnvalue_2 "0, 0, 0" "KeepWorldPosition" true))
  (Niagara|SetNiagaraVariable(Float) _returnvalue_4 "Radius" (Variables|Default|GetbrokenInstrumentRange))
  (bind _returnvalue_5 (Audio|SpawnSoundAttached "/Game/Universal_Systems/Abilities/MetalGuitar_Cue.MetalGuitar_Cue" _returnvalue_3 "None" _returnvalue_2 "0, 0, 0" "KeepWorldPosition" false 1.0 1.0 0.0 0 0))
  (bind _returnvalue_6 (Utilities|Time|SetTimerbyEvent (EventDispatchers|CreateEvent :!event Custom|Stun%20Nearby%20Enemies) 0.15 true))
  (bind _output_get (Variables|Default|SetbrokenInstrumentTimer _returnvalue_6))
  (Utilities|FlowControl|RetriggerableDelay 7.0) ; How long it lasts
  (Utilities|Time|ClearandInvalidateTimerbyHandle _output_get)
  (Audio|Components|Audio|Stop _returnvalue_5)
  (Components|Activation|Deactivate _returnvalue_4))

(event Custom|Stun%20Nearby%20Enemies
  ;[1 0.7373 0] Stun
  (CallFunction|EffectCharactersinRange (Variables|Default|GetbrokenInstrumentRange) "NewEnumerator0"))

(event Custom|Confuse%20Nearby%20Enemies
  ;[0.3854 0 0.3324] Confuse
  (CallFunction|EffectCharactersinRange (Variables|Default|GetconfuseRange) "NewEnumerator1"))

(event Custom|Invisible
  (bind _returnvalue (Utilities|Time|SetTimerbyEvent (EventDispatchers|CreateEvent :!event Custom|Confuse%20Nearby%20Enemies) 0.15 true))
  (bind _output_get (Variables|Default|SetinvisibleTimer _returnvalue))
  (Utilities|FlowControl|RetriggerableDelay 5.0) ; How long it lasts
  (Utilities|Time|ClearandInvalidateTimerbyHandle _output_get))

(fn EffectCharactersinRange
  (params (radius :type Float%20%28double-precision%29) (effectType :type E_EffectType%20Enum :default "NewEnumerator0"))
  (bind _returnvalue (Components|GetOwner))
  (bind _returnvalue_2 (Transformation|GetActorLocation _returnvalue))
  (bind _outhits (Collision|MultiSphereTraceForObjects _returnvalue_2 _returnvalue_2 radius (Utilities|Array|MakeArray "ObjectTypeQuery3") false 0 "None"))
  (for _array_element _outhits
    (if (== (Utilities|Array|FindItem (Variables|Default|GethitActorsArray) 0) -1) ; (Characters get hit more than once,\nthis ensures their event is only activated\nonce per trace)
      (if (Class|GameplayStatics|ObjectIsA (.HitActor (Collision|BreakHitResult _array_element)) "/Game/Characters/Enemy/BP_Character_Enemy.BP_Character_Enemy_C")
        (Utilities|Array|AddUnique (Variables|Default|GethitActorsArray) (.HitActor (Collision|BreakHitResult _array_element)))
        (bind _asbp_character_base (Utilities|Casting|CastToBP_Character_Base (.HitActor (Collision|BreakHitResult _array_element))))
        (switch Utilities|FlowControl|Switch|SwitchonE_EffectType effectType
          (:NewEnumerator0
            (Default|Stunned _asbp_character_base))
          (:NewEnumerator1
            (Default|Confused _asbp_character_base))))))
  (Utilities|Array|Clear (Variables|Default|GethitActorsArray)) ; Clears all actors so they can be\nactivated on the next trace
)