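; BP_KillBox is a kill volume actor that triggers player death when the PlayerCart overlaps it.
; It caches player 0's BP_Character_Player1 on BeginPlay and calls its OnDeath when the overlapping actor matches PlayerCart.
; Older respawn logic for player and cart is left disconnected, and RestartTheGame is an empty event.
; A RespawnActors function exposes the RespawnPoint and PlayerCart references.
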(event Custom|RestartTheGame)

(event EventBeginPlay
  (bind _asbp_character_player_1 (Utilities|Casting|CastToBP_Character_Player1 (Game|GetPlayerCharacter 0))) ; REPLACE WITH PROPER CAST WHEN MERGE
  (Variables|Default|SetAs%20BP%20Character%20Player%201 _asbp_character_player_1))

(event Collision|EventActorBeginOverlap
  (params (OtherActor :type Actor%20Object%20Reference))
  (if (== OtherActor (Variables|Default|GetPlayerCart))
    ;[1 1 1] Delayed Reset (UI CODE GOES HERE)
    (Default|OnDeath (Variables|Default|GetAs%20BP%20Character%20Player%201))))

(event EventTick
  (params (DeltaSeconds :type Float%20%28single-precision%29)))

(fn ConstructionScript)

(fn RespawnActors
  (return (Variables|Default|GetRespawnPoint) (Variables|Default|GetPlayerCart)))