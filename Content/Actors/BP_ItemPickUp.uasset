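; Item pickup actor that rolls one of eight cart power-up types at random on BeginPlay, such as Turret, Plow or Bomb Boost.
; Every type currently uses the same placeholder cube mesh.
; When a possessed pawn overlaps the collision box, it stores that pawn as the player cart, prints the item name and destroys itself.
; Applying items to the cart is not implemented yet.
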(event OnComponentBeginOverlap(CollisionBox)
  (params (OverlappedComponent :type Primitive%20Component%20Object%20Reference) (OtherActor :type Actor%20Object%20Reference) (OtherComp :type Primitive%20Component%20Object%20Reference) (OtherBodyIndex :type Integer) (bFromSweep :type Boolean) (SweepResult :type Hit%20Result%20Structure%20%28by%20ref%29))
  (bind _aspawn (Utilities|Casting|CastToPawn OtherActor))
  (Utilities|IsValid (Pawn|GetController _aspawn)
    (:Is%20Valid
      ;[1 1 1] Items will be plugged in here using the player cart reference to apply items to the cart.
      (Variables|Default|SetPlayerCart _aspawn)
      (switch int (Variables|Default|GetItemType)
        (:0
          (Development|PrintString "Turret"))
        (:1
          (Development|PrintString "Invisibility Potion"))
        (:2
          (Development|PrintString "Explosive Pumpkin"))
        (:3
          (Development|PrintString "Plow"))
        (:4
          (Development|PrintString "Broken Instrument"))
        (:5
          (Development|PrintString "Umbrella"))
        (:6
          (Development|PrintString "Shrinking / enlargement potion"))
        (:7
          (Development|PrintString "Bomb Boost")))
      (Actor|DestroyActor))))

(event Collision|EventActorBeginOverlap
  (params (OtherActor :type Actor%20Object%20Reference)))

(event EventTick
  (params (DeltaSeconds :type Float%20%28single-precision%29)))

(event EventBeginPlay
  (bind _itemmesh (Variables|Default|GetItemMesh))
  (bind _output_get (Variables|Default|SetItemType (Math|Random|RandomIntegerinRange 0 7)))
  (switch int _output_get
    (:0
      (Components|StaticMesh|SetStaticMesh _itemmesh "/Game/StarterContent/Shapes/Shape_Cube.Shape_Cube") ; Turret
    )
    (:1
      (Components|StaticMesh|SetStaticMesh _itemmesh "/Game/StarterContent/Shapes/Shape_Cube.Shape_Cube") ; Invisibilty Potion
    )
    (:2
      (Components|StaticMesh|SetStaticMesh _itemmesh "/Game/StarterContent/Shapes/Shape_Cube.Shape_Cube") ; Explosive Pumpkin
    )
    (:3
      (Components|StaticMesh|SetStaticMesh _itemmesh "/Game/StarterContent/Shapes/Shape_Cube.Shape_Cube") ; Plow
    )
    (:4
      (Components|StaticMesh|SetStaticMesh _itemmesh "/Game/StarterContent/Shapes/Shape_Cube.Shape_Cube") ; Broken Instrument
    )
    (:5
      (Components|StaticMesh|SetStaticMesh _itemmesh "/Game/StarterContent/Shapes/Shape_Cube.Shape_Cube") ; Umbrella
    )
    (:6
      (Components|StaticMesh|SetStaticMesh _itemmesh "/Game/StarterContent/Shapes/Shape_Cube.Shape_Cube") ; Shrinking Enlargement potion
    )
    (:7
      (Components|StaticMesh|SetStaticMesh _itemmesh "/Game/StarterContent/Shapes/Shape_Cube.Shape_Cube") ; Bomb Boost
    )))

(fn ConstructionScript)